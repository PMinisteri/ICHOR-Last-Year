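; Ichor actor that shows an animated, pulsing energy effect with glowing lights.
; BeginPlay loops two skeletal animations, starts timelines that replay after a pause, and destroys the Ichor component.
; The timelines drive material parameter collections and the sphere and green energy light intensities.
; The green light timeline restarts on every update of the material timeline, so it only plays through once that one stops.
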(event EventBeginPlay
  (Utilities|FlowControl|Sequence
    (:then_0
      (Components|Animation|PlayAnimation (Variables|Default|GetIchor+anim_pSphere1) "/Game/PFE/Imports/ICHOR/Animations/Ichor+anim_pSphere101_Anim.Ichor+anim_pSphere101_Anim" true)
      (Components|Animation|PlayAnimation (Variables|Default|GetIchor+anim_C1) "/Game/PFE/Imports/ICHOR/Animations/Ichor+anim_C1_Anim.Ichor+anim_C1_Anim" true))
    (:then_1
      (bind _timeline_ichor (Timeline|Timeline_0 PlayFromStart)
        (:Update
          (Rendering|Material|SetScalarParameterValue "/Game/PFE/Imports/ICHOR/BP/Param_ICHOR_material.Param_ICHOR_material" "Intensity" _timeline_ichor :!class /Script/Engine.KismetMaterialLibrary)
          (bind _timeline_green_light_ichor (Timeline|Timeline_1 PlayFromStart)
            (:Update
              (Rendering|Material|SetScalarParameterValue "/Game/PFE/Imports/ICHOR/BP/Param_pointLight.Param_pointLight" "Intensity" _timeline_green_light_ichor :!class /Script/Engine.KismetMaterialLibrary)
              (Rendering|Components|Light|SetIntensity (Variables|Default|GetGreeneEnergy_light) _timeline_green_light_ichor))))
        (:Finished
          (Utilities|FlowControl|Delay 3.0)
          (Timeline|Timeline_0 PlayFromStart))))
    (:then_2
      (bind _sphere_ichor_pintlight (Timeline|Point_light PlayFromStart)
        (:Update
          (Rendering|Components|Light|SetIntensity (Variables|Default|GetSphere_light) _sphere_ichor_pintlight))
        (:Finished
          (Utilities|FlowControl|Delay 3.0)
          (Timeline|Point_light PlayFromStart))))
    (:then_3
      (Components|DestroyComponent (Variables|Default|Getichor)))))

(event Collision|EventActorBeginOverlap
  (params (OtherActor :type Actor%20Object%20Reference)))

(event EventTick
  (params (DeltaSeconds :type Float%20%28single-precision%29)))

(fn ConstructionScript)