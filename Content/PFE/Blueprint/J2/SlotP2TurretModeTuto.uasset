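; SlotP2TurretModeTuto is a trigger volume that shows a widget to Player 2, apparently a turret mode tutorial prompt.
; When an actor tagged Player2 begins overlapping the Box, it finds the first Player2 actor in the world and makes its Widget2 component visible.
; The end overlap event hides the same widget, without propagating the visibility change to children.
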(event OnComponentBeginOverlap(Box)
  (params (OverlappedComponent :type Primitive%20Component%20Object%20Reference) (OtherActor :type Actor%20Object%20Reference) (OtherComp :type Primitive%20Component%20Object%20Reference) (OtherBodyIndex :type Integer) (bFromSweep :type Boolean) (SweepResult :type Hit%20Result%20Structure%20%28by%20ref%29))
  (if (Actor|ActorHasTag OtherActor "Player2")
    (bind _outactors (Actor|GetAllActorsOfClass "/Game/PFE/Blueprint/J2/Player2.Player2_C"))
    (Rendering|SetVisibility (Variables|/Game/PFE/Blueprint/J2/Player2.Player2_C|GetWidget2 (Utilities|Array|Get(acopy) _outactors)) true false)))

(event OnComponentEndOverlap(Box)
  (params (OverlappedComponent :type Primitive%20Component%20Object%20Reference) (OtherActor :type Actor%20Object%20Reference) (OtherComp :type Primitive%20Component%20Object%20Reference) (OtherBodyIndex :type Integer))
  (if (Actor|ActorHasTag OtherActor "Player2")
    (bind _outactors (Actor|GetAllActorsOfClass "/Game/PFE/Blueprint/J2/Player2.Player2_C"))
    (Rendering|SetVisibility (Variables|/Game/PFE/Blueprint/J2/Player2.Player2_C|GetWidget2 (Utilities|Array|Get(acopy) _outactors)) false false)))

(fn ConstructionScript)