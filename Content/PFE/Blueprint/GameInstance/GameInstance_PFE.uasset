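; Game Instance for the PFE game, holding game-wide state for weapon choice, life, shield, objective life and wave progress.
; Events join a selected multiplayer session, toggle Sword or Claw exclusively, reset stats and wave flags, and play an enemy alert sound at a location.
; SpawnSquareFormation spawns one AI pawn per call in a grid, deriving its offset through division and modulo, and returns an incremented counter.
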(event Custom|Reset
  (Variables|Default|SetObjectifLife 1e+03)
  (CallFunction|ResetWave)
  (Variables|Default|SetShield 1e+03)
  (Variables|Default|SetLife 1e+03))

(event Custom|ResetWave
  (Variables|Wave|SetW1 true)
  (Variables|Wave|SetW2 false)
  (Variables|Wave|SetW3 false)
  (Variables|Wave|SetW4 false)
  (Variables|Wave|SetW5 false)
  (Variables|Wave|SetW6 false)
  (Variables|Wave|SetW7 false)
  (Variables|Wave|SetW8 false)
  (Variables|Wave|SetInW1 false)
  (Variables|Wave|SetInW2 false)
  (Variables|Wave|SetInW3 false)
  (Variables|Wave|SetInW4 false)
  (Variables|Wave|SetFinishWaves false)
  (Variables|Default|SetInTimer false)
  (Variables|Wave|SetInW5 false)
  (Variables|Default|SetInTuto false)
  (Variables|Wave|SetW9 false)
  (Variables|Wave|SetInW5 false)
  (Variables|Wave|SetInW6 false)
  (Variables|Wave|SetInW7 false)
  (Variables|Wave|SetInW8 false)
  (Variables|Wave|SetInW9 false))

(event Custom|ChangeToClaw
  (Variables|Default|SetClaw true)
  (Variables|Default|SetSword false))

(event Custom|ChangeToSword
  (Variables|Default|SetSword true)
  (Variables|Default|SetClaw false))

(event Custom|JoinToSelectedServer
  (params (SearchResult :type Blueprint%20Session%20Result%20Structure%20%28by%20ref%29))
  (|JoinSession (Game|GetPlayerController 0) SearchResult))

(event Custom|Pouet
  (params (Location :type Vector))
  (Audio|PlaySoundatLocation "/Game/PFE/Blueprint/AI/AIGlobal/AlerteEnnemis_Cue.AlerteEnnemis_Cue" Location "0, 0, 0" 1.0 1.0 0.0 0 0 0))

(fn OnRepChargingCrystals)

(fn SpawnSquareFormation
  (params (InputPin :type Integer%20%28by%20ref%29) (InputPin1 :type Pawn%20Class%20Reference) (InputPin2 :type Integer) (InputPin3 :type Integer) (InputPin4 :type Float%20%28single-precision%29) (InputPin5 :type Float%20%28single-precision%29) (InVec :type Vector) (InVec1 :type Vector) (BehaviorTree :type Behavior%20Tree%20Object%20Reference))
  (bind (_x _y _z) (Math|Vector|BreakVector InVec))
  (bind (_x_2 _y_2 _z_2) (Math|Vector|BreakVector InVec1))
  (AI|SpawnAIFromClass InputPin1 BehaviorTree (Math|Vector|MakeVector (+ _x (+ (/ _x_2 2.0) (* InputPin5 (- (Math|Conversions|ToFloat(Integer) (/ InputPin2 InputPin3)) (+ (Math|Conversions|ToFloat(Integer) (/ InputPin3 2)) (* (Math|Integer|%(Integer) InputPin3 2) 0.5)))))) (+ _y (+ (/ _y_2 2.0) (* InputPin4 (Math|Conversions|ToFloat(Integer) (Math|Integer|%(Integer) InputPin2 InputPin3))))) (+ _z _z_2)) "0, 0, 0" false)
  (bind _result (Math|Integer|IncrementInt InputPin)
    (:%20%20
      (return true _result))))