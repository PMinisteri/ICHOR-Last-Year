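; VR multiplayer game mode that starts the enemy wave spawners when play begins.
; BeginPlay caches GameInstance_PFE, then takes the first actor of each spawner class, from the base and 1BIS spawners through wave 9.
; It starts looping named-function timers on all of them at once, with no sequencing here.
; Intervals are the inverse of EnemiesPerSeconds, except 1BIS, which uses the raw value.
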(event EventBeginPlay
  ;[1 1 1] WaveGestion
  (Utilities|FlowControl|Sequence
    (:then_0
      (bind _asgame_instance_pfe (Utilities|Casting|CastToGameInstance_PFE (Game|GetGameInstance)))
      (Variables|Default|SetGI _asgame_instance_pfe))
    (:then_1
      (Utilities|FlowControl|Sequence
        (:then_0
          (bind _outactors (Actor|GetAllActorsOfClass "/Game/PFE/Blueprint/AI/AIGlobal/Spawner/EnemySpawner.EnemySpawner_C"))
          (bind _output_get (Variables|Default|SetSpawner (Utilities|Array|Get(acopy) _outactors)))
          (Utilities|Time|SetTimerbyFunctionName _output_get "SpawnEnemy" (/ 1.0 (Variables|Default|GetEnemiesPerSeconds)) true)
          (bind _outactors_2 (Actor|GetAllActorsOfClass "/Game/PFE/Blueprint/AI/AIGlobal/Spawner/EnemySpawner1BIS.EnemySpawner1BIS_C"))
          (bind _output_get_2 (Variables|Default|SetSpawner1BIS (Utilities|Array|Get(acopy) _outactors_2)))
          (Utilities|Time|SetTimerbyFunctionName _output_get_2 "SpawnEnemy" (Variables|Default|GetEnemiesPerSeconds) true))
        (:then_1
          (bind _outactors_3 (Actor|GetAllActorsOfClass "/Game/PFE/Blueprint/AI/AIGlobal/Spawner/EnemySpawnerW2.EnemySpawnerW2_C"))
          (bind _output_get_3 (Variables|Default|SetSpawnerW2 (Utilities|Array|Get(acopy) _outactors_3)))
          (Utilities|Time|SetTimerbyFunctionName _output_get_3 "Wave2" (/ 1.0 (Variables|Default|GetEnemiesPerSeconds)) true))
        (:then_2
          (bind _outactors_4 (Actor|GetAllActorsOfClass "/Game/PFE/Blueprint/AI/AIGlobal/Spawner/EnemySpawnerW3.EnemySpawnerW3_C"))
          (bind _output_get_4 (Variables|Default|SetSpawner3 (Utilities|Array|Get(acopy) _outactors_4)))
          (Utilities|Time|SetTimerbyFunctionName _output_get_4 "Wave3" (/ 1.0 (Variables|Default|GetEnemiesPerSeconds)) true))
        (:then_3
          (bind _outactors_5 (Actor|GetAllActorsOfClass "/Game/PFE/Blueprint/AI/AIGlobal/Spawner/EnemySpawnerW4.EnemySpawnerW4_C"))
          (bind _output_get_5 (Variables|Default|SetSpawner4 (Utilities|Array|Get(acopy) _outactors_5)))
          (Utilities|Time|SetTimerbyFunctionName _output_get_5 "Wave4" (/ 1.0 (Variables|Default|GetEnemiesPerSeconds)) true))
        (:then_4
          (bind _outactors_6 (Actor|GetAllActorsOfClass "/Game/PFE/Blueprint/AI/AIGlobal/Spawner/EnemySpawnerW5.EnemySpawnerW5_C"))
          (bind _output_get_6 (Variables|Default|SetSpawner5 (Utilities|Array|Get(acopy) _outactors_6)))
          (Utilities|Time|SetTimerbyFunctionName _output_get_6 "Wave5" (/ 1.0 (Variables|Default|GetEnemiesPerSeconds)) true))
        (:then_5
          (bind _outactors_7 (Actor|GetAllActorsOfClass "/Game/PFE/Blueprint/AI/AIGlobal/Spawner/EnemySpawnerW6.EnemySpawnerW6_C"))
          (bind _output_get_7 (Variables|Default|SetSpawner6 (Utilities|Array|Get(acopy) _outactors_7)))
          (Utilities|Time|SetTimerbyFunctionName _output_get_7 "Wave6" (/ 1.0 (Variables|Default|GetEnemiesPerSeconds)) true))
        (:then_6
          (bind _outactors_8 (Actor|GetAllActorsOfClass "/Game/PFE/Blueprint/AI/AIGlobal/Spawner/EnemySpawnerW7.EnemySpawnerW7_C"))
          (bind _output_get_8 (Variables|Default|SetSpawner7_1 (Utilities|Array|Get(acopy) _outactors_8)))
          (Utilities|Time|SetTimerbyFunctionName _output_get_8 "Wave7" (/ 1.0 (Variables|Default|GetEnemiesPerSeconds)) true))
        (:then_7
          (bind _outactors_9 (Actor|GetAllActorsOfClass "/Game/PFE/Blueprint/AI/AIGlobal/Spawner/EnemySpawnerW8.EnemySpawnerW8_C"))
          (bind _output_get_9 (Variables|Default|SetSpawner8 (Utilities|Array|Get(acopy) _outactors_9)))
          (Utilities|Time|SetTimerbyFunctionName _output_get_9 "Wave8" (/ 1.0 (Variables|Default|GetEnemiesPerSeconds)) true))
        (:then_8
          (bind _outactors_10 (Actor|GetAllActorsOfClass "/Game/PFE/Blueprint/AI/AIGlobal/Spawner/EnemySpawnerW9.EnemySpawnerW9_C"))
          (bind _output_get_10 (Variables|Default|SetSpawner9 (Utilities|Array|Get(acopy) _outactors_10)))
          (Utilities|Time|SetTimerbyFunctionName _output_get_10 "Wave9" (/ 1.0 (Variables|Default|GetEnemiesPerSeconds)) true))))))

(fn ConstructionScript)