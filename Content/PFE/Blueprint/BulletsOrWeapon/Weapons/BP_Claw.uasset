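; BP_Claw is a claw weapon that damages what it hits, geared toward destructible actors.
; Overlapping an AI-tagged actor only spawns a hit particle, with no location set.
; The Hit event skips AI-tagged actors and fires one shared chain of radial, point and destructible damage plus a debug print up to three times.
; Two paths require a DestructibleActor cast, while RadialDamage enters the chain past it.
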(event Custom|DamageDM
  (bind _returnvalue (Math|Random|RandomFloatinRange 1e+02 1e+02))
  (bind _staticmesh (Variables|Default|GetStaticMesh))
  (bind _returnvalue_2 (Components|GetOwner _staticmesh))
  (bind _asdestructible_actor (Utilities|Casting|CastToDestructibleActor (.HitActor (Collision|BreakHitResult (stale Collision|EventHit Hit)))))
  (Game|Damage|ApplyRadialDamage 1e+01 (.ImpactPoint (Collision|BreakHitResult (stale Collision|EventHit Hit))) 5e+01 "/Script/Engine.DamageType" 0 _returnvalue_2 0 true "ECC_Visibility")
  (Game|Damage|ApplyPointDamage (.HitActor (Collision|BreakHitResult (stale Collision|EventHit Hit))) _returnvalue (.ImpactPoint (Collision|BreakHitResult (stale Collision|EventHit Hit))) (stale Collision|EventHit Hit) 0 _returnvalue_2)
  (Class|DestructibleComponent|ApplyDamage (Variables|/Script/ApexDestruction.DestructibleActor|GetDestructibleComponent _asdestructible_actor) _returnvalue (.ImpactPoint (Collision|BreakHitResult (stale Collision|EventHit Hit))) (* (.ImpactNormal (Collision|BreakHitResult (stale Collision|EventHit Hit))) -1) 1e+02)
  (Development|PrintText (Utilities|Text|FormatText "Hit {Actor} - Damages : {Damages}" (Utilities|Text|ToText(String) (Utilities|String|ToString(Object) (.HitActor (Collision|BreakHitResult (stale Collision|EventHit Hit))))) (Utilities|Text|ToText(Float) _returnvalue "HalfToEven"))))

(event Custom|Radial%20Damage
  (bind _returnvalue (Math|Random|RandomFloatinRange 1e+02 1e+02))
  (bind _staticmesh (Variables|Default|GetStaticMesh))
  (bind _returnvalue_2 (Components|GetOwner _staticmesh))
  (Game|Damage|ApplyRadialDamage 1e+01 (.ImpactPoint (Collision|BreakHitResult (stale Collision|EventHit Hit))) 5e+01 "/Script/Engine.DamageType" 0 _returnvalue_2 0 true "ECC_Visibility")
  (Game|Damage|ApplyPointDamage (.HitActor (Collision|BreakHitResult (stale Collision|EventHit Hit))) _returnvalue (.ImpactPoint (Collision|BreakHitResult (stale Collision|EventHit Hit))) (stale Collision|EventHit Hit) 0 _returnvalue_2)
  (Class|DestructibleComponent|ApplyDamage (Variables|/Script/ApexDestruction.DestructibleActor|GetDestructibleComponent (stale Custom|DamageDM _asdestructible_actor)) _returnvalue (.ImpactPoint (Collision|BreakHitResult (stale Collision|EventHit Hit))) (* (.ImpactNormal (Collision|BreakHitResult (stale Collision|EventHit Hit))) -1) 1e+02)
  (Development|PrintText (Utilities|Text|FormatText "Hit {Actor} - Damages : {Damages}" (Utilities|Text|ToText(String) (Utilities|String|ToString(Object) (.HitActor (Collision|BreakHitResult (stale Collision|EventHit Hit))))) (Utilities|Text|ToText(Float) _returnvalue "HalfToEven"))))

(event EventBeginPlay
  (|CallParentFunction) ; This node is disabled and will not be called.\nDrag off pins to build functionality.
)

(event Collision|EventHit
  (params (MyComp :type Primitive%20Component%20Object%20Reference) (Other :type Actor%20Object%20Reference) (OtherComp :type Primitive%20Component%20Object%20Reference) (bSelfMoved :type Boolean) (HitLocation :type Vector :default "0, 0, 0") (HitNormal :type Vector :default "0, 0, 0") (NormalImpulse :type Vector :default "0, 0, 0") (Hit :type Hit%20Result%20Structure%20%28by%20ref%29))
  (bind (_bblockinghit _binitialoverlap _time _distance _location _impactpoint _normal _impactnormal _physmat _hitactor) (Collision|BreakHitResult Hit))
  (bind _returnvalue (Math|Random|RandomFloatinRange 1e+02 1e+02))
  (bind _staticmesh (Variables|Default|GetStaticMesh))
  (bind _returnvalue_2 (Components|GetOwner _staticmesh))
  (if (not (Actor|ActorHasTag _hitactor "AI"))
    (Utilities|FlowControl|Sequence
      (:then_0
        (bind _asdestructible_actor (Utilities|Casting|CastToDestructibleActor _hitactor))
        (Game|Damage|ApplyRadialDamage 1e+01 _impactpoint 5e+01 "/Script/Engine.DamageType" 0 _returnvalue_2 0 true "ECC_Visibility")
        (Game|Damage|ApplyPointDamage _hitactor _returnvalue _impactpoint Hit 0 _returnvalue_2)
        (Class|DestructibleComponent|ApplyDamage (Variables|/Script/ApexDestruction.DestructibleActor|GetDestructibleComponent _asdestructible_actor) _returnvalue _impactpoint (* _impactnormal -1) 1e+02)
        (Development|PrintText (Utilities|Text|FormatText "Hit {Actor} - Damages : {Damages}" (Utilities|Text|ToText(String) (Utilities|String|ToString(Object) _hitactor)) (Utilities|Text|ToText(Float) _returnvalue "HalfToEven"))))
      (:then_1
        (CallFunction|DamageDM))
      (:then_2
        (CallFunction|RadialDamage)))))

(event EventTick
  (params (DeltaSeconds :type Float%20%28single-precision%29))
  (|CallParentFunction DeltaSeconds) ; This node is disabled and will not be called.\nDrag off pins to build functionality.
)

(event Collision|EventActorBeginOverlap
  (params (OtherActor :type Actor%20Object%20Reference))
  (if (Actor|ActorHasTag OtherActor "AI")
    (Effects|SpawnEmitteratLocation "/Game/FXVarietyPack/Particles/P_ky_hit2.P_ky_hit2" "0, 0, 0")))

(fn ConstructionScript
  (|CallParentFunction))