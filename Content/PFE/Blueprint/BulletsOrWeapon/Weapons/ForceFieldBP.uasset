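; Force field actor that plays a timed shield material effect on spawn, then removes itself.
; On BeginPlay, Portal1 waits briefly, creates a dynamic Forceshield material on the Plane, and drives its "amount" parameter with a timeline.
; The timeline's update also starts the delay that destroys the actor.
; Sphere hits and the Shoot event share a Laser cast that only prints debug text.
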(event OnComponentHit(Sphere)
  (params (HitComponent :type Primitive%20Component%20Object%20Reference) (OtherActor :type Actor%20Object%20Reference) (OtherComp :type Primitive%20Component%20Object%20Reference) (NormalImpulse :type Vector :default "0, 0, 0") (Hit :type Hit%20Result%20Structure%20%28by%20ref%29))
  (bind _aslaser (Utilities|Casting|CastToLaser OtherActor))
  (Development|PrintString (Utilities|GetDisplayName _aslaser))
  (Development|PrintString "Hello"))

(event Custom|Portal1
  (Utilities|FlowControl|Delay 1.0)
  (bind _returnvalue (Rendering|Material|CreateDynamicMaterialInstance (Variables|Default|GetPlane) 0 "/Game/PFE/Material/Shield/forceshield_M_Inst.forceshield_M_Inst" "None" :!class /Script/Engine.PrimitiveComponent))
  (bind _newtrack_0 (Timeline|Timeline_0 Play)
    (:Update
      (Rendering|Material|SetScalarParameterValue _returnvalue "amount" _newtrack_0 :!class /Script/Engine.MaterialInstanceDynamic)
      (Utilities|FlowControl|Delay 1.9)
      (Actor|DestroyActor))))

(event Custom|Shoot
  (bind _aslaser (Utilities|Casting|CastToLaser (stale OnComponentHit(Sphere) OtherActor)))
  (Development|PrintString (Utilities|GetDisplayName _aslaser))
  (Development|PrintString "Hello"))

(event EventBeginPlay
  (CallFunction|Portal1))

(fn ConstructionScript)