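; Enemy AI character that spawns a rifle in its hand and fires LaserIA shots in a gated, retriggerable-delay loop once PawnSensing spots a BP_WorldInteractionPawn.
; Overlaps on its capsule, mesh and sphere subtract Life by tag (lasers, claw, sword, shock), with surviving hits briefly enabling custom-depth highlighting.
; Death launches the body with physics, dissolves its materials through timelines, increments the GameInstance AI score and destroys rifle and actor.
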(event OnComponentBeginOverlap(CapsuleComponent)
  (params (OverlappedComponent :type Primitive%20Component%20Object%20Reference) (OtherActor :type Actor%20Object%20Reference) (OtherComp :type Primitive%20Component%20Object%20Reference) (OtherBodyIndex :type Integer) (bFromSweep :type Boolean) (SweepResult :type Hit%20Result%20Structure%20%28by%20ref%29))
  (bind _gi (Variables|Default|GetGI))
  (bind _mesh (Variables|Character|GetMesh))
  ;[1 1 1] Take Damage / Die
  (if (Actor|ActorHasTag (stale Collision|EventActorBeginOverlap OtherActor) "Laser")
    (Variables|Default|SetLife (- (Variables|Default|GetLife) 15.0))
    (if (<= (Variables|Default|GetLife) 0.0) :!label _label
      (Physics|SetSimulatePhysics (Variables|Character|GetMesh) true)
      (Physics|AddImpulse (Variables|Collision|GetCapsuleComponent) "10000.000000,10000.000000,10000.000000" "None" false)
      (Collision|SetCollisionEnabled (Variables|Collision|GetCapsuleComponent) "QueryAndPhysics" :!label _label_2)
      (Utilities|FlowControl|Delay 7.0)
      (bind _returnvalue (Rendering|Material|CreateDynamicMaterialInstance (Variables|Character|GetMesh) 0 "/Game/PFE/Material/FX/Disint/MaterialDissolve.MaterialDissolve" "None" :!class /Script/Engine.PrimitiveComponent))
      (Variables|Default|SetIsdead true)
      (bind _newtrack_0 (Timeline|Timeline_0 Play)
        (:Update
          (Rendering|Material|SetScalarParameterValue _returnvalue "Amount" _newtrack_0 :!class /Script/Engine.MaterialInstanceDynamic)
          (bind _returnvalue_2 (Rendering|Material|CreateDynamicMaterialInstance (Variables|Character|GetMesh) 1 "/Game/PFE/Material/FX/Disint/MaterialDissolve.MaterialDissolve" "None" :!class /Script/Engine.PrimitiveComponent))
          (bind _newtrack_0_2 (Timeline|Timeline_1 Play)
            (:Update
              (Rendering|Material|SetScalarParameterValue _returnvalue_2 "amount" _newtrack_0_2 :!class /Script/Engine.MaterialInstanceDynamic)
              (Variables|/Game/PFE/Blueprint/GameInstance/GameInstance_PFE.GameInstance_PFE_C|SetScoreAI _gi (+ (Variables|/Game/PFE/Blueprint/GameInstance/GameInstance_PFE.GameInstance_PFE_C|GetScoreAI _gi) 1))
              (Utilities|FlowControl|Delay 1.5)
              (Actor|DestroyActor (Variables|Default|GetRifle))
              (Actor|DestroyActor)))))
      (else
        ;;[1 0.04918 0] HitScan
        (Rendering|SetRenderCustomDepth _mesh true)
        (Rendering|SetCustomDepthStencilValue (Variables|Character|GetMesh) 2)
        (Utilities|FlowControl|Delay 3.0)
        (Rendering|SetRenderCustomDepth _mesh false)
        (Rendering|SetCustomDepthStencilValue _mesh 2)))
    (elif (or (Actor|ActorHasTag (stale Collision|EventActorBeginOverlap OtherActor) "LaserVR") (Actor|ActorHasTag (stale Collision|EventActorBeginOverlap OtherActor) "LaserTurret"))
      (Variables|Default|SetLife (- (Variables|Default|GetLife) 3e+01))
      (goto _label)
      (elif (not (Actor|ActorHasTag (stale Collision|EventActorBeginOverlap OtherActor) "Scan"))
        (if (or (Actor|ActorHasTag (stale Collision|EventActorBeginOverlap OtherActor) "Claw") (Components|ComponentHasTag OtherComp "Sword"))
          (Variables|Default|SetLife (- (Variables|Default|GetLife) 1e+02))
          (goto _label)
          (elif (Actor|ActorHasTag (stale Collision|EventActorBeginOverlap OtherActor) "Shock")
            (Physics|SetSimulatePhysics (Variables|Character|GetMesh) true)
            (Physics|AddImpulse (Variables|Collision|GetCapsuleComponent) "600.000000,600.000000,600.000000" "None" false)
            (Variables|Default|SetLife (- (Variables|Default|GetLife) (Variables|Default|GetLife)))
            (goto _label_2)
            (elif (Actor|ActorHasTag (stale Collision|EventActorBeginOverlap OtherActor) "DeathAI")
              (CallFunction|DIE))))))))

(event OnComponentBeginOverlap(Sphere)
  (params (OverlappedComponent :type Primitive%20Component%20Object%20Reference) (OtherActor :type Actor%20Object%20Reference) (OtherComp :type Primitive%20Component%20Object%20Reference) (OtherBodyIndex :type Integer) (bFromSweep :type Boolean) (SweepResult :type Hit%20Result%20Structure%20%28by%20ref%29))
  (bind _gi (Variables|Default|GetGI))
  (bind _mesh (Variables|Character|GetMesh))
  ;[1 1 1] Take Damage / Die
  (if (Actor|ActorHasTag OtherActor "Laser")
    (Variables|Default|SetLife (- (Variables|Default|GetLife) 3e+01))
    (if (<= (Variables|Default|GetLife) 0.0) :!label _label
      (Physics|SetSimulatePhysics (Variables|Character|GetMesh) true)
      (Physics|AddImpulse (Variables|Collision|GetCapsuleComponent) "10000.000000,10000.000000,10000.000000" "None" false)
      (Collision|SetCollisionEnabled (Variables|Collision|GetCapsuleComponent) "QueryAndPhysics")
      (Utilities|FlowControl|Delay 7.0)
      (bind _returnvalue (Rendering|Material|CreateDynamicMaterialInstance (Variables|Character|GetMesh) 0 "/Game/PFE/Material/FX/Disint/MaterialDissolve.MaterialDissolve" "None" :!class /Script/Engine.PrimitiveComponent))
      (Variables|Default|SetIsdead true)
      (bind _newtrack_0 (Timeline|Timeline_0 Play)
        (:Update
          (Rendering|Material|SetScalarParameterValue _returnvalue "Amount" _newtrack_0 :!class /Script/Engine.MaterialInstanceDynamic)
          (bind _returnvalue_2 (Rendering|Material|CreateDynamicMaterialInstance (Variables|Character|GetMesh) 1 "/Game/PFE/Material/FX/Disint/MaterialDissolve.MaterialDissolve" "None" :!class /Script/Engine.PrimitiveComponent))
          (bind _newtrack_0_2 (Timeline|Timeline_1 Play)
            (:Update
              (Rendering|Material|SetScalarParameterValue _returnvalue_2 "amount" _newtrack_0_2 :!class /Script/Engine.MaterialInstanceDynamic)
              (Variables|/Game/PFE/Blueprint/GameInstance/GameInstance_PFE.GameInstance_PFE_C|SetScoreAI _gi (+ (Variables|/Game/PFE/Blueprint/GameInstance/GameInstance_PFE.GameInstance_PFE_C|GetScoreAI _gi) 1))
              (Utilities|FlowControl|Delay 1.5)
              (Actor|DestroyActor (Variables|Default|GetRifle))
              (Actor|DestroyActor)))))
      (else
        ;;[1 0.04918 0] HitScan
        (Rendering|SetRenderCustomDepth _mesh true)
        (Rendering|SetCustomDepthStencilValue (Variables|Character|GetMesh) 2)
        (Utilities|FlowControl|Delay 3.0)
        (Rendering|SetRenderCustomDepth _mesh false)
        (Rendering|SetCustomDepthStencilValue _mesh 2)))
    (elif (Actor|ActorHasTag OtherActor "LaserTurret")
      (Variables|Default|SetLife (- (Variables|Default|GetLife) 1e+02))
      (goto _label))))

(event OnComponentBeginOverlap(Mesh)
  (params (OverlappedComponent :type Primitive%20Component%20Object%20Reference) (OtherActor :type Actor%20Object%20Reference) (OtherComp :type Primitive%20Component%20Object%20Reference) (OtherBodyIndex :type Integer) (bFromSweep :type Boolean) (SweepResult :type Hit%20Result%20Structure%20%28by%20ref%29))
  (bind _gi (Variables|Default|GetGI))
  (bind _mesh (Variables|Character|GetMesh))
  ;[1 1 1] Take Damage / Die
  (if (Actor|ActorHasTag (stale Collision|EventActorBeginOverlap OtherActor) "Laser")
    (Variables|Default|SetLife (- (Variables|Default|GetLife) 15.0))
    (if (<= (Variables|Default|GetLife) 0.0) :!label _label
      (Physics|SetSimulatePhysics (Variables|Character|GetMesh) true)
      (Physics|AddImpulse (Variables|Collision|GetCapsuleComponent) "10000.000000,10000.000000,10000.000000" "None" false)
      (Collision|SetCollisionEnabled (Variables|Collision|GetCapsuleComponent) "QueryAndPhysics" :!label _label_2)
      (Utilities|FlowControl|Delay 7.0)
      (bind _returnvalue (Rendering|Material|CreateDynamicMaterialInstance (Variables|Character|GetMesh) 0 "/Game/PFE/Material/FX/Disint/MaterialDissolve.MaterialDissolve" "None" :!class /Script/Engine.PrimitiveComponent))
      (Variables|Default|SetIsdead true)
      (bind _newtrack_0 (Timeline|Timeline_0 Play)
        (:Update
          (Rendering|Material|SetScalarParameterValue _returnvalue "Amount" _newtrack_0 :!class /Script/Engine.MaterialInstanceDynamic)
          (bind _returnvalue_2 (Rendering|Material|CreateDynamicMaterialInstance (Variables|Character|GetMesh) 1 "/Game/PFE/Material/FX/Disint/MaterialDissolve.MaterialDissolve" "None" :!class /Script/Engine.PrimitiveComponent))
          (bind _newtrack_0_2 (Timeline|Timeline_1 Play)
            (:Update
              (Rendering|Material|SetScalarParameterValue _returnvalue_2 "amount" _newtrack_0_2 :!class /Script/Engine.MaterialInstanceDynamic)
              (Variables|/Game/PFE/Blueprint/GameInstance/GameInstance_PFE.GameInstance_PFE_C|SetScoreAI _gi (+ (Variables|/Game/PFE/Blueprint/GameInstance/GameInstance_PFE.GameInstance_PFE_C|GetScoreAI _gi) 1))
              (Utilities|FlowControl|Delay 1.5)
              (Actor|DestroyActor (Variables|Default|GetRifle))
              (Actor|DestroyActor)))))
      (else
        ;;[1 0.04918 0] HitScan
        (Rendering|SetRenderCustomDepth _mesh true)
        (Rendering|SetCustomDepthStencilValue (Variables|Character|GetMesh) 2)
        (Utilities|FlowControl|Delay 3.0)
        (Rendering|SetRenderCustomDepth _mesh false)
        (Rendering|SetCustomDepthStencilValue _mesh 2)))
    (elif (or (Actor|ActorHasTag (stale Collision|EventActorBeginOverlap OtherActor) "LaserVR") (Actor|ActorHasTag (stale Collision|EventActorBeginOverlap OtherActor) "LaserTurret"))
      (Variables|Default|SetLife (- (Variables|Default|GetLife) 3e+01))
      (goto _label)
      (elif (not (Actor|ActorHasTag (stale Collision|EventActorBeginOverlap OtherActor) "Scan"))
        (if (or (Actor|ActorHasTag (stale Collision|EventActorBeginOverlap OtherActor) "Claw") (Components|ComponentHasTag (stale OnComponentBeginOverlap(CapsuleComponent) OtherComp) "Sword"))
          (Variables|Default|SetLife (- (Variables|Default|GetLife) 1e+02))
          (goto _label)
          (elif (Actor|ActorHasTag (stale Collision|EventActorBeginOverlap OtherActor) "Shock")
            (Physics|SetSimulatePhysics (Variables|Character|GetMesh) true)
            (Physics|AddImpulse (Variables|Collision|GetCapsuleComponent) "600.000000,600.000000,600.000000" "None" false)
            (Variables|Default|SetLife (- (Variables|Default|GetLife) (Variables|Default|GetLife)))
            (goto _label_2)
            (elif (Actor|ActorHasTag (stale Collision|EventActorBeginOverlap OtherActor) "DeathAI")
              (CallFunction|DIE))))))))

(event OnSeePawn(PawnSensing)
  (params (Pawn :type Pawn%20Object%20Reference))
  (Utilities|Casting|CastToBP_WorldInteractionPawn Pawn)
  (CallFunction|FoundEnemy))

(event Custom|Challenge1
  (bind _gi (Variables|Default|GetGI))
  ;[1 1 1] Take Damage / Die
  (if (Variables|/Game/PFE/Blueprint/GameInstance/GameInstance_PFE.GameInstance_PFE_C|GetChallenge1Active _gi)
    (Variables|/Game/PFE/Blueprint/GameInstance/GameInstance_PFE.GameInstance_PFE_C|SetChallenge1EnemyKill _gi (+ (Variables|/Game/PFE/Blueprint/GameInstance/GameInstance_PFE.GameInstance_PFE_C|GetChallenge1EnemyKill _gi) 1.0))
    (if (>= (Variables|/Game/PFE/Blueprint/GameInstance/GameInstance_PFE.GameInstance_PFE_C|GetChallenge1EnemyKill _gi) 1.0)
      (Variables|/Game/PFE/Blueprint/GameInstance/GameInstance_PFE.GameInstance_PFE_C|SetChallenge1Valid (Variables|Default|GetGI) true))))

(event Custom|Ragdoll
  (bind _returnvalue (Utilities|Name|MakeLiteralName "pelvis"))
  (bind _mesh (Variables|Character|GetMesh))
  (Utilities|FlowControl|Sequence
    (:then_0
      (Class|SkeletalMeshComponent|SetAllBodiesBelowSimulatePhysics _mesh _returnvalue true true)
      (Class|SkeletalMeshComponent|SetAllBodiesBelowPhysicsBlendWeight _mesh _returnvalue 1.0 false true)
      (Variables|Default|SetInRagdoll true))
    (:then_1
      (Utilities|FlowControl|Delay 2.0)
      (Class|SkeletalMeshComponent|SetAllBodiesBelowSimulatePhysics (Variables|Character|GetMesh) _returnvalue false true)
      (Variables|Default|SetInRagdoll false)
      (Transformation|AttachComponentToComponent (Variables|Character|GetMesh) (Variables|Collision|GetCapsuleComponent) "None" "SnapToTarget" "SnapToTarget" "KeepWorld" true)
      (Transformation|SetRelativeLocationAndRotation (Variables|Character|GetMesh) "0, 0,-97.000000" "0,-90.000000, 0" false false))))

(event Custom|DIE
  (Actor|DestroyActor))

(event Custom|Death
  (bind _gi (Variables|Default|GetGI))
  ;[1 1 1] Take Damage / Die
  (Physics|SetSimulatePhysics (Variables|Character|GetMesh) true)
  (Physics|AddImpulse (Variables|Collision|GetCapsuleComponent) "10000.000000,10000.000000,10000.000000" "None" false)
  (Collision|SetCollisionEnabled (Variables|Collision|GetCapsuleComponent) "QueryAndPhysics")
  (Utilities|FlowControl|Delay 7.0)
  (bind _returnvalue (Rendering|Material|CreateDynamicMaterialInstance (Variables|Character|GetMesh) 0 "/Game/PFE/Material/FX/Disint/MaterialDissolve.MaterialDissolve" "None" :!class /Script/Engine.PrimitiveComponent))
  (Variables|Default|SetIsdead true)
  (bind _newtrack_0 (Timeline|Timeline_0 Play)
    (:Update
      (Rendering|Material|SetScalarParameterValue _returnvalue "Amount" _newtrack_0 :!class /Script/Engine.MaterialInstanceDynamic)
      (bind _returnvalue_2 (Rendering|Material|CreateDynamicMaterialInstance (Variables|Character|GetMesh) 1 "/Game/PFE/Material/FX/Disint/MaterialDissolve.MaterialDissolve" "None" :!class /Script/Engine.PrimitiveComponent))
      (bind _newtrack_0_2 (Timeline|Timeline_1 Play)
        (:Update
          (Rendering|Material|SetScalarParameterValue _returnvalue_2 "amount" _newtrack_0_2 :!class /Script/Engine.MaterialInstanceDynamic)
          (Variables|/Game/PFE/Blueprint/GameInstance/GameInstance_PFE.GameInstance_PFE_C|SetScoreAI _gi (+ (Variables|/Game/PFE/Blueprint/GameInstance/GameInstance_PFE.GameInstance_PFE_C|GetScoreAI _gi) 1))
          (Utilities|FlowControl|Delay 1.5)
          (Actor|DestroyActor (Variables|Default|GetRifle))
          (Actor|DestroyActor))))))

(event Custom|EnemyLost
  (Variables|Default|SetFireMode? false)
  (Variables|Default|SetUseRifle false))

(event Custom|FoundEnemy
  (Variables|Default|SetUseRifle true)
  (Variables|Default|SetFireMode? true)
  (Utilities|FlowControl|Sequence
    (:then_0
      (goto _label Open))
    (:then_1
      (Utilities|FlowControl|Gate true :!label _label
        (:Exit
          (Utilities|FlowControl|Sequence
            (:then_0
              (if (Variables|Default|GetFireMode?)
                (Variables|Default|SetFire true)
                (CallFunction|FireBullet)))
            (:then_1
              (Utilities|FlowControl|RetriggerableDelay 0.2)
              (goto _label))))))))

(event EventBeginPlay
  (Utilities|FlowControl|Sequence
    (:then_0
      (bind _asgame_instance_pfe (Utilities|Casting|CastToGameInstance_PFE (Game|GetGameInstance)))
      (Variables|Default|SetGI _asgame_instance_pfe)
      (bind _outactors (Actor|GetAllActorsOfClass "/Game/PFE/Blueprint/J2/Player2.Player2_C"))
      (Variables|Default|SetP2 (Utilities|Array|Get(acopy) _outactors)))
    (:then_1
      (Variables|Default|SetAIControllerClass "/Game/PFE/Blueprint/AI/AIRefonte/AICharacterContDef.AICharacterContDef_C")
      (CallFunction|AttachRifle))))

(event EventTick
  (params (DeltaSeconds :type Float%20%28single-precision%29)))

(event Collision|EventActorBeginOverlap
  (params (OtherActor :type Actor%20Object%20Reference))
  (bind _gi (Variables|Default|GetGI))
  (bind _mesh (Variables|Character|GetMesh))
  ;[1 1 1] Take Damage / Die
  (if (Actor|ActorHasTag OtherActor "Laser")
    (Variables|Default|SetLife (- (Variables|Default|GetLife) 15.0))
    (if (<= (Variables|Default|GetLife) 0.0) :!label _label
      (Physics|SetSimulatePhysics (Variables|Character|GetMesh) true)
      (Physics|AddImpulse (Variables|Collision|GetCapsuleComponent) "10000.000000,10000.000000,10000.000000" "None" false)
      (Collision|SetCollisionEnabled (Variables|Collision|GetCapsuleComponent) "QueryAndPhysics" :!label _label_2)
      (Utilities|FlowControl|Delay 7.0)
      (bind _returnvalue (Rendering|Material|CreateDynamicMaterialInstance (Variables|Character|GetMesh) 0 "/Game/PFE/Material/FX/Disint/MaterialDissolve.MaterialDissolve" "None" :!class /Script/Engine.PrimitiveComponent))
      (Variables|Default|SetIsdead true)
      (bind _newtrack_0 (Timeline|Timeline_0 Play)
        (:Update
          (Rendering|Material|SetScalarParameterValue _returnvalue "Amount" _newtrack_0 :!class /Script/Engine.MaterialInstanceDynamic)
          (bind _returnvalue_2 (Rendering|Material|CreateDynamicMaterialInstance (Variables|Character|GetMesh) 1 "/Game/PFE/Material/FX/Disint/MaterialDissolve.MaterialDissolve" "None" :!class /Script/Engine.PrimitiveComponent))
          (bind _newtrack_0_2 (Timeline|Timeline_1 Play)
            (:Update
              (Rendering|Material|SetScalarParameterValue _returnvalue_2 "amount" _newtrack_0_2 :!class /Script/Engine.MaterialInstanceDynamic)
              (Variables|/Game/PFE/Blueprint/GameInstance/GameInstance_PFE.GameInstance_PFE_C|SetScoreAI _gi (+ (Variables|/Game/PFE/Blueprint/GameInstance/GameInstance_PFE.GameInstance_PFE_C|GetScoreAI _gi) 1))
              (Utilities|FlowControl|Delay 1.5)
              (Actor|DestroyActor (Variables|Default|GetRifle))
              (Actor|DestroyActor)))))
      (else
        ;;[1 0.04918 0] HitScan
        (Rendering|SetRenderCustomDepth _mesh true)
        (Rendering|SetCustomDepthStencilValue (Variables|Character|GetMesh) 2)
        (Utilities|FlowControl|Delay 3.0)
        (Rendering|SetRenderCustomDepth _mesh false)
        (Rendering|SetCustomDepthStencilValue _mesh 2)))
    (elif (or (Actor|ActorHasTag OtherActor "LaserVR") (Actor|ActorHasTag OtherActor "LaserTurret"))
      (Variables|Default|SetLife (- (Variables|Default|GetLife) 3e+01))
      (goto _label)
      (elif (not (Actor|ActorHasTag OtherActor "Scan"))
        (if (or (Actor|ActorHasTag OtherActor "Claw") (Components|ComponentHasTag (stale OnComponentBeginOverlap(CapsuleComponent) OtherComp) "Sword"))
          (Variables|Default|SetLife (- (Variables|Default|GetLife) 1e+02))
          (goto _label)
          (elif (Actor|ActorHasTag OtherActor "Shock")
            (Physics|SetSimulatePhysics (Variables|Character|GetMesh) true)
            (Physics|AddImpulse (Variables|Collision|GetCapsuleComponent) "600.000000,600.000000,600.000000" "None" false)
            (Variables|Default|SetLife (- (Variables|Default|GetLife) (Variables|Default|GetLife)))
            (goto _label_2)
            (elif (Actor|ActorHasTag OtherActor "DeathAI")
              (CallFunction|DIE))))))))

(fn ConstructionScript)

(fn AttachRifle
  (bind _returnvalue (Game|SpawnActorfromClass "/Game/RifleBP.RifleBP_C" (Transformation|GetActorTransform) "Undefined" 0 0))
  (bind _output_get (Variables|Default|SetRifle _returnvalue))
  (Transformation|AttachComponentToComponent _output_get (Variables|Character|GetMesh) "Rifle_hand" "SnapToTarget" "SnapToTarget" "SnapToTarget" true))

(fn FireBullet
  (bind _mesh (Variables|Character|GetMesh))
  (Game|SpawnActorfromClass "/Game/PFE/Blueprint/BulletsOrWeapon/Bullets/LaserIA.LaserIA_C" (Math|Transform|MakeTransform (Transformation|GetSocketLocation _mesh "Rifle_bullet") (Math|Rotator|MakeRotator 0.0 0.0 (.Yaw (Math|Rotator|BreakRotator (Transformation|GetSocketRotation _mesh "Rifle_bullet"))))) "AlwaysSpawn" 0 0))