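; AI controller for IA_Enemy pawns that patrols a waypoint route in a back-and-forth loop.
; BeginPlay caches the pawn and its waypoints, then Patrolling re-calls itself after each successful AIMoveTo until FoundEnemy is set.
; The hunt trigger using FocusP2 and IsDead is disconnected, leaving the looping CheckEnemy timer empty and OnHunt's chase of the player unused.
; Fire is only an uncalled debug line trace.
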(event Custom|Fire
  (Collision|LineTraceByChannel "0, 0, 0" "0, 0, 0" "TraceTypeQuery1" true 0 "ForDuration"))

(event Custom|Patrolling
  (if (not (Variables|Default|GetFoundEnemy))
    (if (Variables|Default|GetWalkBack)
      (Math|Integer|DecrementInt (Variables|Default|GetCurrentWaypoint)
        (:%20%20
          (AI|AIMoveTo 0 "0, 0, 0" (Utilities|Array|Get(acopy) (Variables|Default|GetWaypoints) (Variables|Default|GetCurrentWaypoint)) 5.0 false
            (:OnSuccess
              (if (<= (Variables|Default|GetCurrentWaypoint) 0)
                (Variables|Default|SetWalkBack false))))))
      (else
        (Math|Integer|IncrementInt (Variables|Default|GetCurrentWaypoint)
          (:%20%20
            (AI|AIMoveTo 0 "0, 0, 0" (Utilities|Array|Get(acopy) (Variables|Default|GetWaypoints) (Variables|Default|GetCurrentWaypoint)) 5.0 false
              (:OnSuccess
                (if (>= (Variables|Default|GetCurrentWaypoint) (- (Utilities|Array|Length (Variables|Default|GetWaypoints)) 1))
                  (Variables|Default|SetWalkBack true))))))))
    (CallFunction|Patrolling)))

(event Custom|OnHunt
  (AI|AIMoveTo 0 "0, 0, 0" (Game|GetPlayerCharacter 0) 1e+03 false))

(event Custom|CheckEnemy)

(event EventBeginPlay
  (bind _asia_enemy (Utilities|Casting|CastToIA_Enemy (Pawn|GetControlledPawn)))
  (Variables|Default|SetAIBaseRef _asia_enemy)
  (Variables|Default|SetWaypoints (Variables|/Game/PFE/Blueprint/AI/IA_Enemy.IA_Enemy_C|GetWaypoint _asia_enemy))
  (bind _returnvalue (Utilities|Time|SetTimerbyFunctionName 0 "CheckEnemy" 0.3 true))
  (Variables|Default|SetCleanTimer _returnvalue)
  (Utilities|FlowControl|Delay 0.2)
  (AI|AIMoveTo 0 "0, 0, 0" (Utilities|Array|Get(acopy) (Variables|Default|GetWaypoints) (Variables|Default|GetCurrentWaypoint)) 5.0 false
    (:OnSuccess
      (CallFunction|Patrolling))))

(fn ConstructionScript)