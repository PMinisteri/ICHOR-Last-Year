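; Base enemy character that takes tag-based overlap damage from lasers, claws, swords and shocks, and can ragdoll temporarily.
; Non-lethal hits flash a custom-depth highlight; death applies physics and impulse, dissolves materials through timelines, raises the GameInstance AI score, then destroys the actor.
; Ragdoll simulates bodies below the pelvis while Tick keeps the capsule following the mesh.
; Helper functions compute objective formation offsets; weapon, light and challenge logic is disconnected.
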(event OnComponentBeginOverlap(CapsuleComponent)
  (params (OverlappedComponent :type Primitive%20Component%20Object%20Reference) (OtherActor :type Actor%20Object%20Reference) (OtherComp :type Primitive%20Component%20Object%20Reference) (OtherBodyIndex :type Integer) (bFromSweep :type Boolean) (SweepResult :type Hit%20Result%20Structure%20%28by%20ref%29))
  (bind _gi (Variables|Default|GetGI))
  (bind _skeletalmesh (Variables|Default|GetSkeletalMesh))
  (bind _mesh (Variables|Character|GetMesh))
  ;[1 1 1] Take Damage / Die
  (if (Actor|ActorHasTag (stale Collision|EventActorBeginOverlap OtherActor) "Laser")
    (Variables|Default|SetLife (- (Variables|Default|GetLife) 15.0))
    (if (<= (Variables|Default|GetLife) 0.0) :!label _label
      (Physics|SetSimulatePhysics (Variables|Collision|GetCapsuleComponent) true)
      (Physics|AddImpulse (Variables|Collision|GetCapsuleComponent) "10000.000000,10000.000000,10000.000000" "None" false)
      (Collision|SetCollisionEnabled (Variables|Collision|GetCapsuleComponent) "QueryAndPhysics" :!label _label_2)
      (Utilities|FlowControl|Delay 0.0)
      (bind _returnvalue (Rendering|Material|CreateDynamicMaterialInstance _skeletalmesh 0 "/Game/PFE/Material/FX/Disint/MaterialDissolve.MaterialDissolve" "None" :!class /Script/Engine.PrimitiveComponent))
      (Variables|Default|SetIsdead true)
      (bind _newtrack_0 (Timeline|Timeline_0 Play)
        (:Update
          (Rendering|Material|SetScalarParameterValue _returnvalue "Amount" _newtrack_0 :!class /Script/Engine.MaterialInstanceDynamic)
          (bind _returnvalue_2 (Rendering|Material|CreateDynamicMaterialInstance _skeletalmesh 1 "/Game/PFE/Material/FX/Disint/MaterialDissolve.MaterialDissolve" "None" :!class /Script/Engine.PrimitiveComponent))
          (bind _newtrack_0_2 (Timeline|Timeline_1 Play)
            (:Update
              (Rendering|Material|SetScalarParameterValue _returnvalue_2 "amount" _newtrack_0_2 :!class /Script/Engine.MaterialInstanceDynamic)
              (Variables|/Game/PFE/Blueprint/GameInstance/GameInstance_PFE.GameInstance_PFE_C|SetScoreAI _gi (+ (Variables|/Game/PFE/Blueprint/GameInstance/GameInstance_PFE.GameInstance_PFE_C|GetScoreAI _gi) 1))
              (Utilities|FlowControl|Delay 1.5)
              (Actor|DestroyActor)))))
      (else
        ;;[1 0.04918 0] HitScan
        (Rendering|SetRenderCustomDepth _mesh true)
        (Rendering|SetCustomDepthStencilValue (Variables|Character|GetMesh) 2)
        (Utilities|FlowControl|Delay 3.0)
        (Rendering|SetRenderCustomDepth _mesh false)
        (Rendering|SetCustomDepthStencilValue _mesh 2)))
    (elif (or (Actor|ActorHasTag (stale Collision|EventActorBeginOverlap OtherActor) "LaserVR") (Actor|ActorHasTag (stale Collision|EventActorBeginOverlap OtherActor) "LaserTurret"))
      (Variables|Default|SetLife (- (Variables|Default|GetLife) 3e+01))
      (goto _label)
      (elif (not (Actor|ActorHasTag (stale Collision|EventActorBeginOverlap OtherActor) "Scan"))
        (if (or (Actor|ActorHasTag (stale Collision|EventActorBeginOverlap OtherActor) "Claw") (Components|ComponentHasTag OtherComp "Sword"))
          (Variables|Default|SetLife (- (Variables|Default|GetLife) 1e+02))
          (goto _label)
          (elif (Actor|ActorHasTag (stale Collision|EventActorBeginOverlap OtherActor) "Shock")
            (Physics|SetSimulatePhysics (Variables|Character|GetMesh) true)
            (Physics|AddImpulse (Variables|Collision|GetCapsuleComponent) "600.000000,600.000000,600.000000" "None" false)
            (Variables|Default|SetLife (- (Variables|Default|GetLife) (Variables|Default|GetLife)))
            (goto _label_2)
            (elif (Actor|ActorHasTag (stale Collision|EventActorBeginOverlap OtherActor) "DeathAI")
              (CallFunction|DIE))))))))

(event OnComponentBeginOverlap(Sphere)
  (params (OverlappedComponent :type Primitive%20Component%20Object%20Reference) (OtherActor :type Actor%20Object%20Reference) (OtherComp :type Primitive%20Component%20Object%20Reference) (OtherBodyIndex :type Integer) (bFromSweep :type Boolean) (SweepResult :type Hit%20Result%20Structure%20%28by%20ref%29))
  (bind _gi (Variables|Default|GetGI))
  (bind _skeletalmesh (Variables|Default|GetSkeletalMesh))
  (bind _mesh (Variables|Character|GetMesh))
  ;[1 1 1] Take Damage / Die
  (if (Actor|ActorHasTag OtherActor "Laser")
    (Variables|Default|SetLife (- (Variables|Default|GetLife) 3e+01))
    (if (<= (Variables|Default|GetLife) 0.0) :!label _label
      (Physics|SetSimulatePhysics (Variables|Collision|GetCapsuleComponent) true)
      (Physics|AddImpulse (Variables|Collision|GetCapsuleComponent) "10000.000000,10000.000000,10000.000000" "None" false)
      (Collision|SetCollisionEnabled (Variables|Collision|GetCapsuleComponent) "QueryAndPhysics")
      (Utilities|FlowControl|Delay 0.0)
      (bind _returnvalue (Rendering|Material|CreateDynamicMaterialInstance _skeletalmesh 0 "/Game/PFE/Material/FX/Disint/MaterialDissolve.MaterialDissolve" "None" :!class /Script/Engine.PrimitiveComponent))
      (Variables|Default|SetIsdead true)
      (bind _newtrack_0 (Timeline|Timeline_0 Play)
        (:Update
          (Rendering|Material|SetScalarParameterValue _returnvalue "Amount" _newtrack_0 :!class /Script/Engine.MaterialInstanceDynamic)
          (bind _returnvalue_2 (Rendering|Material|CreateDynamicMaterialInstance _skeletalmesh 1 "/Game/PFE/Material/FX/Disint/MaterialDissolve.MaterialDissolve" "None" :!class /Script/Engine.PrimitiveComponent))
          (bind _newtrack_0_2 (Timeline|Timeline_1 Play)
            (:Update
              (Rendering|Material|SetScalarParameterValue _returnvalue_2 "amount" _newtrack_0_2 :!class /Script/Engine.MaterialInstanceDynamic)
              (Variables|/Game/PFE/Blueprint/GameInstance/GameInstance_PFE.GameInstance_PFE_C|SetScoreAI _gi (+ (Variables|/Game/PFE/Blueprint/GameInstance/GameInstance_PFE.GameInstance_PFE_C|GetScoreAI _gi) 1))
              (Utilities|FlowControl|Delay 1.5)
              (Actor|DestroyActor)))))
      (else
        ;;[1 0.04918 0] HitScan
        (Rendering|SetRenderCustomDepth _mesh true)
        (Rendering|SetCustomDepthStencilValue (Variables|Character|GetMesh) 2)
        (Utilities|FlowControl|Delay 3.0)
        (Rendering|SetRenderCustomDepth _mesh false)
        (Rendering|SetCustomDepthStencilValue _mesh 2)))
    (elif (Actor|ActorHasTag OtherActor "LaserTurret")
      (Variables|Default|SetLife (- (Variables|Default|GetLife) 1e+02))
      (goto _label))))

(event OnComponentBeginOverlap(Mesh)
  (params (OverlappedComponent :type Primitive%20Component%20Object%20Reference) (OtherActor :type Actor%20Object%20Reference) (OtherComp :type Primitive%20Component%20Object%20Reference) (OtherBodyIndex :type Integer) (bFromSweep :type Boolean) (SweepResult :type Hit%20Result%20Structure%20%28by%20ref%29))
  (bind _gi (Variables|Default|GetGI))
  (bind _skeletalmesh (Variables|Default|GetSkeletalMesh))
  (bind _mesh (Variables|Character|GetMesh))
  ;[1 1 1] Take Damage / Die
  (if (Actor|ActorHasTag (stale Collision|EventActorBeginOverlap OtherActor) "Laser")
    (Variables|Default|SetLife (- (Variables|Default|GetLife) 15.0))
    (if (<= (Variables|Default|GetLife) 0.0) :!label _label
      (Physics|SetSimulatePhysics (Variables|Collision|GetCapsuleComponent) true)
      (Physics|AddImpulse (Variables|Collision|GetCapsuleComponent) "10000.000000,10000.000000,10000.000000" "None" false)
      (Collision|SetCollisionEnabled (Variables|Collision|GetCapsuleComponent) "QueryAndPhysics" :!label _label_2)
      (Utilities|FlowControl|Delay 0.0)
      (bind _returnvalue (Rendering|Material|CreateDynamicMaterialInstance _skeletalmesh 0 "/Game/PFE/Material/FX/Disint/MaterialDissolve.MaterialDissolve" "None" :!class /Script/Engine.PrimitiveComponent))
      (Variables|Default|SetIsdead true)
      (bind _newtrack_0 (Timeline|Timeline_0 Play)
        (:Update
          (Rendering|Material|SetScalarParameterValue _returnvalue "Amount" _newtrack_0 :!class /Script/Engine.MaterialInstanceDynamic)
          (bind _returnvalue_2 (Rendering|Material|CreateDynamicMaterialInstance _skeletalmesh 1 "/Game/PFE/Material/FX/Disint/MaterialDissolve.MaterialDissolve" "None" :!class /Script/Engine.PrimitiveComponent))
          (bind _newtrack_0_2 (Timeline|Timeline_1 Play)
            (:Update
              (Rendering|Material|SetScalarParameterValue _returnvalue_2 "amount" _newtrack_0_2 :!class /Script/Engine.MaterialInstanceDynamic)
              (Variables|/Game/PFE/Blueprint/GameInstance/GameInstance_PFE.GameInstance_PFE_C|SetScoreAI _gi (+ (Variables|/Game/PFE/Blueprint/GameInstance/GameInstance_PFE.GameInstance_PFE_C|GetScoreAI _gi) 1))
              (Utilities|FlowControl|Delay 1.5)
              (Actor|DestroyActor)))))
      (else
        ;;[1 0.04918 0] HitScan
        (Rendering|SetRenderCustomDepth _mesh true)
        (Rendering|SetCustomDepthStencilValue (Variables|Character|GetMesh) 2)
        (Utilities|FlowControl|Delay 3.0)
        (Rendering|SetRenderCustomDepth _mesh false)
        (Rendering|SetCustomDepthStencilValue _mesh 2)))
    (elif (or (Actor|ActorHasTag (stale Collision|EventActorBeginOverlap OtherActor) "LaserVR") (Actor|ActorHasTag (stale Collision|EventActorBeginOverlap OtherActor) "LaserTurret"))
      (Variables|Default|SetLife (- (Variables|Default|GetLife) 3e+01))
      (goto _label)
      (elif (not (Actor|ActorHasTag (stale Collision|EventActorBeginOverlap OtherActor) "Scan"))
        (if (or (Actor|ActorHasTag (stale Collision|EventActorBeginOverlap OtherActor) "Claw") (Components|ComponentHasTag (stale OnComponentBeginOverlap(CapsuleComponent) OtherComp) "Sword"))
          (Variables|Default|SetLife (- (Variables|Default|GetLife) 1e+02))
          (goto _label)
          (elif (Actor|ActorHasTag (stale Collision|EventActorBeginOverlap OtherActor) "Shock")
            (Physics|SetSimulatePhysics (Variables|Character|GetMesh) true)
            (Physics|AddImpulse (Variables|Collision|GetCapsuleComponent) "600.000000,600.000000,600.000000" "None" false)
            (Variables|Default|SetLife (- (Variables|Default|GetLife) (Variables|Default|GetLife)))
            (goto _label_2)
            (elif (Actor|ActorHasTag (stale Collision|EventActorBeginOverlap OtherActor) "DeathAI")
              (CallFunction|DIE))))))))

(event Custom|Challenge1
  (bind _gi (Variables|Default|GetGI))
  ;[1 1 1] Take Damage / Die
  (if (Variables|/Game/PFE/Blueprint/GameInstance/GameInstance_PFE.GameInstance_PFE_C|GetChallenge1Active _gi)
    (Variables|/Game/PFE/Blueprint/GameInstance/GameInstance_PFE.GameInstance_PFE_C|SetChallenge1EnemyKill _gi (+ (Variables|/Game/PFE/Blueprint/GameInstance/GameInstance_PFE.GameInstance_PFE_C|GetChallenge1EnemyKill _gi) 1.0))
    (if (>= (Variables|/Game/PFE/Blueprint/GameInstance/GameInstance_PFE.GameInstance_PFE_C|GetChallenge1EnemyKill _gi) 1.0)
      (Variables|/Game/PFE/Blueprint/GameInstance/GameInstance_PFE.GameInstance_PFE_C|SetChallenge1Valid (Variables|Default|GetGI) true))))

(event Custom|Ragdoll
  (bind _returnvalue (Utilities|Name|MakeLiteralName "pelvis"))
  (bind _mesh (Variables|Character|GetMesh))
  (Utilities|FlowControl|Sequence
    (:then_0
      (Class|SkeletalMeshComponent|SetAllBodiesBelowSimulatePhysics _mesh _returnvalue true true)
      (Class|SkeletalMeshComponent|SetAllBodiesBelowPhysicsBlendWeight _mesh _returnvalue 1.0 false true)
      (Variables|Default|SetInRagdoll true))
    (:then_1
      (Utilities|FlowControl|Delay 2.0)
      (Class|SkeletalMeshComponent|SetAllBodiesBelowSimulatePhysics (Variables|Character|GetMesh) _returnvalue false true)
      (Variables|Default|SetInRagdoll false)
      (Transformation|AttachComponentToComponent (Variables|Character|GetMesh) (Variables|Collision|GetCapsuleComponent) "None" "SnapToTarget" "SnapToTarget" "KeepWorld" true)
      (Transformation|SetRelativeLocationAndRotation (Variables|Character|GetMesh) "0, 0,-97.000000" "0,-90.000000, 0" false false))))

(event Custom|Death
  (bind _gi (Variables|Default|GetGI))
  (bind _skeletalmesh (Variables|Default|GetSkeletalMesh))
  ;[1 1 1] Take Damage / Die
  (Physics|SetSimulatePhysics (Variables|Collision|GetCapsuleComponent) true)
  (Physics|AddImpulse (Variables|Collision|GetCapsuleComponent) "10000.000000,10000.000000,10000.000000" "None" false)
  (Collision|SetCollisionEnabled (Variables|Collision|GetCapsuleComponent) "QueryAndPhysics")
  (Utilities|FlowControl|Delay 0.0)
  (bind _returnvalue (Rendering|Material|CreateDynamicMaterialInstance _skeletalmesh 0 "/Game/PFE/Material/FX/Disint/MaterialDissolve.MaterialDissolve" "None" :!class /Script/Engine.PrimitiveComponent))
  (Variables|Default|SetIsdead true)
  (bind _newtrack_0 (Timeline|Timeline_0 Play)
    (:Update
      (Rendering|Material|SetScalarParameterValue _returnvalue "Amount" _newtrack_0 :!class /Script/Engine.MaterialInstanceDynamic)
      (bind _returnvalue_2 (Rendering|Material|CreateDynamicMaterialInstance _skeletalmesh 1 "/Game/PFE/Material/FX/Disint/MaterialDissolve.MaterialDissolve" "None" :!class /Script/Engine.PrimitiveComponent))
      (bind _newtrack_0_2 (Timeline|Timeline_1 Play)
        (:Update
          (Rendering|Material|SetScalarParameterValue _returnvalue_2 "amount" _newtrack_0_2 :!class /Script/Engine.MaterialInstanceDynamic)
          (Variables|/Game/PFE/Blueprint/GameInstance/GameInstance_PFE.GameInstance_PFE_C|SetScoreAI _gi (+ (Variables|/Game/PFE/Blueprint/GameInstance/GameInstance_PFE.GameInstance_PFE_C|GetScoreAI _gi) 1))
          (Utilities|FlowControl|Delay 1.5)
          (Actor|DestroyActor))))))

(event Custom|DIE
  (Actor|DestroyActor))

(event EventBeginPlay
  (Utilities|FlowControl|Sequence
    (:then_0
      (bind _asgame_instance_pfe (Utilities|Casting|CastToGameInstance_PFE (Game|GetGameInstance)))
      (Variables|Default|SetGI _asgame_instance_pfe)
      (bind _outactors (Actor|GetAllActorsOfClass "/Game/PFE/Blueprint/J2/Player2.Player2_C"))
      (Variables|Default|SetP2 (Utilities|Array|Get(acopy) _outactors)))
    (:then_1
      (CallFunction|AttachWeapon)
      (CallFunction|AttachLights))))

(event EventTick
  (params (DeltaSeconds :type Float%20%28single-precision%29))
  (if (Variables|Default|GetInRagdoll)
    (Transformation|SetWorldLocation (Variables|Collision|GetCapsuleComponent) (+ (Transformation|GetWorldLocation (Variables|Character|GetMesh)) "0, 0,97.000000") false false)))

(event Collision|EventActorBeginOverlap
  (params (OtherActor :type Actor%20Object%20Reference))
  (bind _gi (Variables|Default|GetGI))
  (bind _skeletalmesh (Variables|Default|GetSkeletalMesh))
  (bind _mesh (Variables|Character|GetMesh))
  ;[1 1 1] Take Damage / Die
  (if (Actor|ActorHasTag OtherActor "Laser")
    (Variables|Default|SetLife (- (Variables|Default|GetLife) 15.0))
    (if (<= (Variables|Default|GetLife) 0.0) :!label _label
      (Physics|SetSimulatePhysics (Variables|Collision|GetCapsuleComponent) true)
      (Physics|AddImpulse (Variables|Collision|GetCapsuleComponent) "10000.000000,10000.000000,10000.000000" "None" false)
      (Collision|SetCollisionEnabled (Variables|Collision|GetCapsuleComponent) "QueryAndPhysics" :!label _label_2)
      (Utilities|FlowControl|Delay 0.0)
      (bind _returnvalue (Rendering|Material|CreateDynamicMaterialInstance _skeletalmesh 0 "/Game/PFE/Material/FX/Disint/MaterialDissolve.MaterialDissolve" "None" :!class /Script/Engine.PrimitiveComponent))
      (Variables|Default|SetIsdead true)
      (bind _newtrack_0 (Timeline|Timeline_0 Play)
        (:Update
          (Rendering|Material|SetScalarParameterValue _returnvalue "Amount" _newtrack_0 :!class /Script/Engine.MaterialInstanceDynamic)
          (bind _returnvalue_2 (Rendering|Material|CreateDynamicMaterialInstance _skeletalmesh 1 "/Game/PFE/Material/FX/Disint/MaterialDissolve.MaterialDissolve" "None" :!class /Script/Engine.PrimitiveComponent))
          (bind _newtrack_0_2 (Timeline|Timeline_1 Play)
            (:Update
              (Rendering|Material|SetScalarParameterValue _returnvalue_2 "amount" _newtrack_0_2 :!class /Script/Engine.MaterialInstanceDynamic)
              (Variables|/Game/PFE/Blueprint/GameInstance/GameInstance_PFE.GameInstance_PFE_C|SetScoreAI _gi (+ (Variables|/Game/PFE/Blueprint/GameInstance/GameInstance_PFE.GameInstance_PFE_C|GetScoreAI _gi) 1))
              (Utilities|FlowControl|Delay 1.5)
              (Actor|DestroyActor)))))
      (else
        ;;[1 0.04918 0] HitScan
        (Rendering|SetRenderCustomDepth _mesh true)
        (Rendering|SetCustomDepthStencilValue (Variables|Character|GetMesh) 2)
        (Utilities|FlowControl|Delay 3.0)
        (Rendering|SetRenderCustomDepth _mesh false)
        (Rendering|SetCustomDepthStencilValue _mesh 2)))
    (elif (or (Actor|ActorHasTag OtherActor "LaserVR") (Actor|ActorHasTag OtherActor "LaserTurret"))
      (Variables|Default|SetLife (- (Variables|Default|GetLife) 3e+01))
      (goto _label)
      (elif (not (Actor|ActorHasTag OtherActor "Scan"))
        (if (or (Actor|ActorHasTag OtherActor "Claw") (Components|ComponentHasTag (stale OnComponentBeginOverlap(CapsuleComponent) OtherComp) "Sword"))
          (Variables|Default|SetLife (- (Variables|Default|GetLife) 1e+02))
          (goto _label)
          (elif (Actor|ActorHasTag OtherActor "Shock")
            (Physics|SetSimulatePhysics (Variables|Character|GetMesh) true)
            (Physics|AddImpulse (Variables|Collision|GetCapsuleComponent) "600.000000,600.000000,600.000000" "None" false)
            (Variables|Default|SetLife (- (Variables|Default|GetLife) (Variables|Default|GetLife)))
            (goto _label_2)
            (elif (Actor|ActorHasTag OtherActor "DeathAI")
              (CallFunction|DIE))))))))

(fn ConstructionScript)

(fn AttachWeapon)

(fn AttachLights)

(fn CalculDestinationObjectif()
  (params (Objectif :type Objectives%20Object%20Reference))
  (bind _capsulecomponent (Variables|Collision|GetCapsuleComponent))
  (bind _asobjectives (Utilities|Casting|CastToObjectives Objectif))
  (Variables|Default|SetObjectifesCast _asobjectives)
  (Transformation|SetActorRotation (Math|Rotator|MakeRotator (.roll (Transformation|GetActorRotation (Variables|Default|GetObjectifesCast))) (.pitch (Transformation|GetActorRotation (Variables|Default|GetObjectifesCast))) (.yaw (Math|Rotator|FindLookatRotation (Transformation|GetActorLocation) (Transformation|GetWorldLocation (Variables|/Game/PFE/Blueprint/Multiplayer/Objectives.Objectives_C|GetCube (Variables|Default|GetObjectifesCast)))))))
  (bind _numunit (CallFunction|GetUnitNumberonSide() self))
  (bind _xobjectifoffset (CallFunction|PlaceUnitObjectif() (- _numunit 48)))
  (return (Math|Vector|MakeVector (.x (+ (Transformation|GetWorldLocation _capsulecomponent) (Math|Vector|MakeVector (+ _xobjectifoffset (.x (Math|Transform|InverseTransformLocation (Transformation|GetWorldTransform _capsulecomponent) (Transformation|GetWorldLocation (Variables|/Game/PFE/Blueprint/Multiplayer/Objectives.Objectives_C|GetCube (Variables|Default|GetObjectifesCast)))))) (+ 0.0 (.y (Math|Transform|InverseTransformLocation (Transformation|GetWorldTransform _capsulecomponent) (Transformation|GetWorldLocation (Variables|/Game/PFE/Blueprint/Multiplayer/Objectives.Objectives_C|GetCube (Variables|Default|GetObjectifesCast)))))) (.z (Math|Transform|InverseTransformLocation (Transformation|GetWorldTransform _capsulecomponent) (Transformation|GetWorldLocation (Variables|/Game/PFE/Blueprint/Multiplayer/Objectives.Objectives_C|GetCube (Variables|Default|GetObjectifesCast)))))))) (.y (Math|Transform|InverseTransformLocation (Transformation|GetWorldTransform _capsulecomponent) (Transformation|GetWorldLocation (Variables|/Game/PFE/Blueprint/Multiplayer/Objectives.Objectives_C|GetCube (Variables|Default|GetObjectifesCast))))) (.z (+ (Transformation|GetWorldLocation _capsulecomponent) (Math|Vector|MakeVector (+ _xobjectifoffset (.x (Math|Transform|InverseTransformLocation (Transformation|GetWorldTransform _capsulecomponent) (Transformation|GetWorldLocation (Variables|/Game/PFE/Blueprint/Multiplayer/Objectives.Objectives_C|GetCube (Variables|Default|GetObjectifesCast)))))) (+ 0.0 (.y (Math|Transform|InverseTransformLocation (Transformation|GetWorldTransform _capsulecomponent) (Transformation|GetWorldLocation (Variables|/Game/PFE/Blueprint/Multiplayer/Objectives.Objectives_C|GetCube (Variables|Default|GetObjectifesCast)))))) (.z (Math|Transform|InverseTransformLocation (Transformation|GetWorldTransform _capsulecomponent) (Transformation|GetWorldLocation (Variables|/Game/PFE/Blueprint/Multiplayer/Objectives.Objectives_C|GetCube (Variables|Default|GetObjectifesCast)))))))))))

(fn GetUnitNumberonSide()
  (params (BPBaseEnemyRef :type BP%20Base%20Enemy%20Object%20Reference))
  (bind _returnvalue (Utilities|GetObjectName BPBaseEnemyRef))
  (bind _stringbaseenemy (Variables|Default|GetStringBaseEnemy))
  (bind _rights (Utilities|String|Split _returnvalue _stringbaseenemy))
  (if (Class|KismetStringLibrary|IsNumeric _rights)
    (Variables|Default|SetResultUnitNum (Utilities|String|GetCharacterasNumber _rights))
    (else
      (Variables|Default|SetResultUnitNum 0)))
  (return 0))

(fn PlaceUnitObjectif()
  (params (NumUnit :type Integer))
  (return (* (Math|Integer|%(Integer) (- NumUnit (Variables|Default|GetNumMiddleUnit)) (Variables|Default|GetNumByLine)) (Variables|Default|GetEspacement_Line))))