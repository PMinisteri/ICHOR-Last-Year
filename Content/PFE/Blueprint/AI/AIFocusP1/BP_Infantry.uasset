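; AI infantry enemy that advances on the first Objectives actor and shoots lasers, adding to the AI score at zero life.
; AI Perception flags the player pawn and writes to the Blackboard; Tick then aims the muzzle arrow at random ScopeList points, otherwise moves toward the objective.
; A looping Fire timer shoots when near player or objective, triggering a delayed, Blackboard-synced reload when empty.
; Older movement and formation-placement code remains disconnected.
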(event OnPerceptionUpdated(AIPerception)
  (params (UpdatedActors :type Array%20of%20Actor%20Object%20References))
  ;[1 1 1] Ai Perceptive OnSight
  (bind _info (Class|AIPerceptionComponent|GetActorsPerception (Variables|Default|GetAIPerception) (Utilities|Array|Get(acopy) UpdatedActors)))
  (if (.bSuccessfullySensed (Utilities|Struct|BreakAIStimulus (Utilities|Array|Get(acopy) (.LastSensedStimuli (Utilities|Struct|BreakActorPerceptionBlueprintInfo _info)))))
    (bind _array_element (Utilities|Array|ForEachLoopwithBreak (Class|AIPerceptionComponent|GetCurrentlyPerceivedActors (Variables|Default|GetAIPerception)))
      (:LoopBody
        (AI|Components|Blackboard|SetValueasObject (AI|GetBlackboard 0) (Utilities|Name|MakeLiteralName "TargetToFollow_Tmp") _array_element)
        ;;[1 1 1] To refacto
        (bind _asbp_world_interaction_pawn (Utilities|Casting|CastToBP_WorldInteractionPawn _array_element))
        (Variables|Default|SetSeeP1 (== _asbp_world_interaction_pawn _array_element))
        (Variables|Default|SetSeeTarget (== _asbp_world_interaction_pawn _array_element))))))

(event Custom|Reload
  (if (not (or (Variables|Default|GetIsReloading) (Variables|Default|GetIsdead_0)))
    (AI|Components|Blackboard|SetValueasBool (AI|GetBlackboard (Pawn|GetController)) (Utilities|Name|MakeLiteralName "isReloading") true)
    (Variables|Default|SetIsReloading true)
    (Utilities|FlowControl|Delay 2.5)
    (Variables|Default|SetAmmoInMag (Variables|Default|GetMaxAmmoInMag))
    (Variables|Default|SetIsReloading false)
    (AI|Components|Blackboard|SetValueasBool (AI|GetBlackboard (Pawn|GetController)) (Utilities|Name|MakeLiteralName "isReloading") false)))

(event Custom|Fire
  (if (>= (Variables|Default|GetLife) 1.0)
    (if (<= (Variables|Default|GetAmmoInMag) 0)
      (CallFunction|Reload)
      (elif (or (< (Math|Vector|VectorLength (- (Transformation|GetActorLocation (Game|Player|GetPlayerPawn 0)) (Transformation|GetActorLocation))) 1.5e+03) (<= (Math|Vector|VectorLength (- (Transformation|GetActorLocation (Variables|Default|GetObjectif)) (Transformation|GetActorLocation))) 6e+02))
        (Game|SpawnActorfromClass "/Game/PFE/Blueprint/BulletsOrWeapon/Bullets/LaserIA.LaserIA_C" (Transformation|GetWorldTransform (Variables|Default|GetArrow1)) "Undefined" 0 0)
        (Variables|Default|SetAmmoInMag (- (Variables|Default|GetAmmoInMag) 1))
        (CallFunction|Shoot)))))

(event Custom|TargetP1
  (Transformation|SetWorldRotation (Variables|Default|GetArrow1) (Math|Rotator|FindLookatRotation (Transformation|GetWorldLocation (Variables|Default|GetArrow1)) (Utilities|Array|Get(acopy) (Variables|/Game/PFE/Blueprint/J1/BP_WorldInteractionPawn.BP_WorldInteractionPawn_C|GetScopeList (stale EventTick _asbp_world_interaction_pawn)) (Math|Random|RandomIntegerinRange 0 5))) false false))

(event Custom|GiveScore
  (bind _gi (Variables|Default|GetGI))
  ;[1 1 1] GiveScore
  (if (<= (Variables|Default|GetLife) 0.0)
    (Variables|/Game/PFE/Blueprint/GameInstance/GameInstance_PFE.GameInstance_PFE_C|SetScoreAI _gi (+ (Variables|/Game/PFE/Blueprint/GameInstance/GameInstance_PFE.GameInstance_PFE_C|GetScoreAI _gi) 1))))

(event Custom|Shoot
  (Audio|Components|Audio|Play (Variables|Default|GetAudio) 0.0))

(event Custom|Rotate
  ;[1 1 1] Comment
)

(event Custom|ChaseObjectif
  (if (Variables|Default|GetWalking_0)
    ;[0.1013 1 0] Code JUJU to Refacto
    (AI|AIMoveTo self (Math|Vector|MakeVector (.x (Variables|Default|GetObjectifInfantryCoordonnate_0)) (.y (Variables|Default|GetObjectifInfantryCoordonnate_0)) (.z (Variables|Default|GetObjectifInfantryCoordonnate_0))) (Variables|Default|GetObjectif) 5e+02 false
      (:then
        (Variables|Default|SetWalking_0 true)
        (CallFunction|Rotate)))
    (else
      (bind _destination (Default|CalculDestinationObjectif() self (Variables|Default|GetObjectif)))
      (Variables|Default|SetObjectifInfantryCoordonnate_0 _destination)
      (Variables|Default|SetWalking_0 true))))

(event EventBeginPlay
  ;[1 1 1] BeginPlay
  (Utilities|FlowControl|Sequence
    (:then_0
      (Utilities|Time|SetTimerbyFunctionName 0 "Fire" (Math|Random|RandomFloatinRange 0.3 0.6) true))
    (:then_1
      (Utilities|Time|SetTimerbyFunctionName 0 "GiveScore" 0.0 true))
    (:then_2
      (bind _outactors (Actor|GetAllActorsOfClass "/Game/PFE/Blueprint/Multiplayer/Objectives.Objectives_C"))
      (Variables|Default|SetObjectif (Utilities|Array|Get(acopy) _outactors)))
    (:then_3
      (CallFunction|AttachWeapon))
    (:then_4
      (AI|Components|Blackboard|SetValueasFloat (AI|GetBlackboard 0) (Utilities|Name|MakeLiteralName "LostSightRadius") 8e+02))))

(event EventTick
  (params (DeltaSeconds :type Float%20%28single-precision%29))
  (if (Variables|Default|GetSeeP1)
    (Utilities|FlowControl|Delay 0.2)
    (bind _asbp_world_interaction_pawn (Utilities|Casting|CastToBP_WorldInteractionPawn (Game|Player|GetPlayerPawn 0)))
    (CallFunction|TargetP1)
    (else
      (CallFunction|ChaseObjectif))))

(fn ConstructionScript
  (|CallParentFunction))

(fn Orientto
  (params (Actor :type Actor%20Object%20Reference) (Cible :type Actor%20Object%20Reference))
  (Transformation|SetActorRotation (Math|Interpolation|RInterpTo (Transformation|GetActorRotation Actor) (Math|Rotator|MakeRotator 0.0 0.0 (.Yaw (Math|Rotator|BreakRotator (Math|Rotator|FindLookatRotation (Transformation|GetActorLocation Actor) (Transformation|GetActorLocation Cible))))) (Utilities|Time|GetWorldDeltaSeconds) 5.0)))

(fn GetMiddleUnit()0
  (params (UnitDetected :type BP%20Base%20Enemy%20Object%20Reference))
  (bind _outactors (Actor|GetAllActorsOfClass "/Game/PFE/Blueprint/AI/AIGlobal/BP_BaseEnemy.BP_BaseEnemy_C"))
  (for _array_element _outactors
    (if (Utilities|Enum|Equal(Enum) (Utilities|GetObjectName _array_element) "BP_Infantry_C_2")
      _))
  (return (Math|Vector|GetUpVector (Variables|Transformation|GetRootComponent)) "BP_Infantry_C_2"))

(fn GetUnitNumberonSide()0
  (params (BPBaseEnemyRef :type BP%20Base%20Enemy%20Object%20Reference))
  (bind _returnvalue (Utilities|GetObjectName BPBaseEnemyRef))
  (bind _stringbaseenemy_0 (Variables|Default|GetStringBaseEnemy_0))
  (bind _rights (Utilities|String|Split _returnvalue _stringbaseenemy_0))
  (if (Class|KismetStringLibrary|IsNumeric _rights)
    (Variables|Default|SetResultUnitNum_0 (Utilities|String|GetCharacterasNumber _rights))
    (else
      (Variables|Default|SetResultUnitNum_0 0)))
  (return (Variables|Default|GetResultUnitNum_0)))

(fn PlaceUnitObjectif()0
  (params (NumUnit :type Integer))
  (return (* (Math|Integer|%(Integer) (- NumUnit (Variables|Default|GetNumMiddleUnit_0)) (Variables|Default|GetNumByLine_0)) (Variables|Default|GetEspacement_Line_0))))