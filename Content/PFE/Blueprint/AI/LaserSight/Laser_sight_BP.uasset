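; Laser sight actor that projects a visible beam and red-dot style marker from its LaserCylinder component.
; Each Tick it line-traces on Visibility along the cylinder's forward vector.
; On a hit, it stretches the cylinder's X scale to the impact distance and spawns a very short-lived dot decal oriented to the surface normal, re-spawned every frame rather than moved.
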(event EventTick
  (params (DeltaSeconds :type Float%20%28single-precision%29))
  (CallFunction|LineTraceforLaserSight))

(fn ConstructionScript)

(fn LineTraceforLaserSight
  (bind _laser_cylinder (Variables|Default|Getlaser_cylinder))
  (bind _returnvalue (Transformation|GetWorldLocation _laser_cylinder))
  (bind (_outhit _returnvalue_2) (Collision|LineTraceByChannel _returnvalue (+ _returnvalue (* (Math|Vector|GetForwardVector _laser_cylinder) 8888.0)) "TraceTypeQuery1" false 0 "None" true "(R=1.000000,G=0.000000,B=0.000000,A=1.000000)" "(R=0.000000,G=1.000000,B=0.000000,A=1.000000)" 0.01))
  (if _returnvalue_2
    (Transformation|SetWorldScale3D _laser_cylinder (Math|Vector|MakeVector (/ (Math|Vector|VectorLength (- (.ImpactPoint (Collision|BreakHitResult _outhit)) (.TraceStart (Collision|BreakHitResult _outhit)))) 1e+01) 1.0 1.0))
    (bind _output_get (LocalVariables|SetLocalDirection (.Location (Collision|BreakHitResult _outhit))))
    (Rendering|Decal|SpawnDecalatLocation "/Game/PFE/Blueprint/AI/LaserSight/Dot_Inst.Dot_Inst" "50.000000,50.000000,50.000000" _output_get (Math|Rotator|MakeRotfromX (.Normal (Collision|BreakHitResult _outhit))) 0.01)))