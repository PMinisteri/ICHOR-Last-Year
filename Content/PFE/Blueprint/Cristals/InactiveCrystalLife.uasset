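; InactiveCrystalLife is a dormant crystal that activates once, when an actor tagged "Laser" overlaps it, and turns into a black hole.
; Activation, shared with the RunOnServer2 event, hides the child actor, applies a dynamic crystal material and plays a timeline into an unnamed ("None") scalar parameter.
; A six-second Delay started from timeline updates then spawns Blackhole at the crystal component's transform and destroys that component.
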(event Custom|RunOnServer2
  (Rendering|ToggleVisibility (Variables|Default|GetChildActor) false)
  (Variables|Default|SetActive true)
  (Rendering|Material|SetMaterial (Variables|Default|GetCyrstalLife) 0 "/Game/PFE/Blueprint/Cristals/Materials/Cristals_Inst.Cristals_Inst")
  (bind _returnvalue (Rendering|Material|CreateDynamicMaterialInstance (Variables|Default|GetCyrstalLife) 0 "/Game/PFE/Blueprint/Cristals/Materials/Cristals_Inst.Cristals_Inst" "None" :!class /Script/Engine.PrimitiveComponent))
  (bind _newtrack_0 (Timeline|Timeline_0 Play)
    (:Update
      (Rendering|Material|SetScalarParameterValue _returnvalue "None" _newtrack_0 :!class /Script/Engine.MaterialInstanceDynamic)
      (Utilities|FlowControl|Delay 6.0)
      (Game|SpawnActorfromClass "/Game/PFE/Blueprint/Cristals/Blackhole.Blackhole_C" (Transformation|GetWorldTransform (Variables|Default|GetCyrstalLife)) "Undefined" 0 0)
      (Components|DestroyComponent (Variables|Default|GetCyrstalLife)))))

(event EventBeginPlay
  (bind _asgame_instance_pfe (Utilities|Casting|CastToGameInstance_PFE (Game|GetGameInstance)))
  (Variables|Default|SetGI _asgame_instance_pfe))

(event Collision|EventActorBeginOverlap
  (params (OtherActor :type Actor%20Object%20Reference))
  (if (and (not (Variables|Default|GetActive)) (Actor|ActorHasTag OtherActor "Laser"))
    (Rendering|ToggleVisibility (Variables|Default|GetChildActor) false)
    (Variables|Default|SetActive true)
    (Rendering|Material|SetMaterial (Variables|Default|GetCyrstalLife) 0 "/Game/PFE/Blueprint/Cristals/Materials/Cristals_Inst.Cristals_Inst")
    (bind _returnvalue (Rendering|Material|CreateDynamicMaterialInstance (Variables|Default|GetCyrstalLife) 0 "/Game/PFE/Blueprint/Cristals/Materials/Cristals_Inst.Cristals_Inst" "None" :!class /Script/Engine.PrimitiveComponent))
    (bind _newtrack_0 (Timeline|Timeline_0 Play)
      (:Update
        (Rendering|Material|SetScalarParameterValue _returnvalue "None" _newtrack_0 :!class /Script/Engine.MaterialInstanceDynamic)
        (Utilities|FlowControl|Delay 6.0)
        (Game|SpawnActorfromClass "/Game/PFE/Blueprint/Cristals/Blackhole.Blackhole_C" (Transformation|GetWorldTransform (Variables|Default|GetCyrstalLife)) "Undefined" 0 0)
        (Components|DestroyComponent (Variables|Default|GetCyrstalLife))))))

(fn ConstructionScript)