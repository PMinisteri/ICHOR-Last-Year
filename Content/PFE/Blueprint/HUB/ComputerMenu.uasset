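; Hub computer menu where actors tagged "Hand" overlap button boxes to pick missions, activate a challenge or upgrade either player's life.
; State booleans and delays gate presses, while visibility and collision toggles swap submenus.
; Selecting a mission shows a loading-screen widget and stores a servertravel command, which the Launch button executes.
; Challenge and tiered upgrade state lives in GameInstance_PFE, with upgrades checking Money without deducting it here.
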(event OnComponentBeginOverlap(MissionMenuBox)
  (params (OverlappedComponent :type Primitive%20Component%20Object%20Reference) (OtherActor :type Actor%20Object%20Reference) (OtherComp :type Primitive%20Component%20Object%20Reference) (OtherBodyIndex :type Integer) (bFromSweep :type Boolean) (SweepResult :type Hit%20Result%20Structure%20%28by%20ref%29))
  ;[1 1 1] Press Mission
  (CallFunction|PressMissionButton OtherActor))

(event OnComponentBeginOverlap(LaunchButtonBox)
  (params (OverlappedComponent :type Primitive%20Component%20Object%20Reference) (OtherActor :type Actor%20Object%20Reference) (OtherComp :type Primitive%20Component%20Object%20Reference) (OtherBodyIndex :type Integer) (bFromSweep :type Boolean) (SweepResult :type Hit%20Result%20Structure%20%28by%20ref%29))
  ;[1 1 1] Launch Mission
  (if (and (Actor|ActorHasTag OtherActor "Hand") (Variables|Missions|GetMissionValid))
    (CallFunction|ChangeLevel)))

(event OnComponentBeginOverlap(ValidUpgradeButtonBox)
  (params (OverlappedComponent :type Primitive%20Component%20Object%20Reference) (OtherActor :type Actor%20Object%20Reference) (OtherComp :type Primitive%20Component%20Object%20Reference) (OtherBodyIndex :type Integer) (bFromSweep :type Boolean) (SweepResult :type Hit%20Result%20Structure%20%28by%20ref%29))
  (CallFunction|ValidUpgradeButtonEvent OtherActor))

(event OnComponentBeginOverlap(P2ButtonBox)
  (params (OverlappedComponent :type Primitive%20Component%20Object%20Reference) (OtherActor :type Actor%20Object%20Reference) (OtherComp :type Primitive%20Component%20Object%20Reference) (OtherBodyIndex :type Integer) (bFromSweep :type Boolean) (SweepResult :type Hit%20Result%20Structure%20%28by%20ref%29))
  (CallFunction|PressP2UpgradeButton OtherActor))

(event OnComponentBeginOverlap(Mission0Box)
  (params (OverlappedComponent :type Primitive%20Component%20Object%20Reference) (OtherActor :type Actor%20Object%20Reference) (OtherComp :type Primitive%20Component%20Object%20Reference) (OtherBodyIndex :type Integer) (bFromSweep :type Boolean) (SweepResult :type Hit%20Result%20Structure%20%28by%20ref%29))
  (if (Math|Boolean|ANDBoolean (Actor|ActorHasTag OtherActor "Hand") (Variables|Missions|GetInMissionMenu) (not (Variables|Missions|GetMissionValid)))
    (Variables|Missions|SetMissionValid true)
    (Rendering|SetVisibility (Variables|Default|GetLaunchButton) true false)
    (Rendering|SetVisibility (Variables|Default|GetMission1) false false)
    (Collision|SetCollisionEnabled (Variables|Default|GetUpgradeMenuBox) "NoCollision")
    (Variables|Missions|SetInMissionMenu false)
    (CallFunction|LoadingScreen)
    (Variables|Default|SetMissionToLaunch "servertravel /Game/PFE/Levels/Level_0")))

(event OnComponentBeginOverlap(LiffeUpgradeP2ButtonBox)
  (params (OverlappedComponent :type Primitive%20Component%20Object%20Reference) (OtherActor :type Actor%20Object%20Reference) (OtherComp :type Primitive%20Component%20Object%20Reference) (OtherBodyIndex :type Integer) (bFromSweep :type Boolean) (SweepResult :type Hit%20Result%20Structure%20%28by%20ref%29))
  (CallFunction|PressLifeUpgradeP2Button OtherActor))

(event OnComponentBeginOverlap(Mission1Box)
  (params (OverlappedComponent :type Primitive%20Component%20Object%20Reference) (OtherActor :type Actor%20Object%20Reference) (OtherComp :type Primitive%20Component%20Object%20Reference) (OtherBodyIndex :type Integer) (bFromSweep :type Boolean) (SweepResult :type Hit%20Result%20Structure%20%28by%20ref%29))
  ;[1 1 1] Mission1
  (if (Math|Boolean|ANDBoolean (Actor|ActorHasTag OtherActor "Hand") (Variables|Missions|GetInMissionMenu) (not (Variables|Missions|GetMissionValid)))
    (Variables|Missions|SetMissionValid true)
    (Rendering|SetVisibility (Variables|Default|GetLaunchButton) true false)
    (Rendering|SetVisibility (Variables|Default|GetMission1) false false)
    (Collision|SetCollisionEnabled (Variables|Default|GetUpgradeMenuBox) "NoCollision")
    (Variables|Missions|SetInMissionMenu false)
    (CallFunction|LoadingScreen)
    (Variables|Default|SetMissionToLaunch "servertravel /Game/PFE/Levels/Level_1")))

(event OnComponentBeginOverlap(ChallengeMenuBox)
  (params (OverlappedComponent :type Primitive%20Component%20Object%20Reference) (OtherActor :type Actor%20Object%20Reference) (OtherComp :type Primitive%20Component%20Object%20Reference) (OtherBodyIndex :type Integer) (bFromSweep :type Boolean) (SweepResult :type Hit%20Result%20Structure%20%28by%20ref%29))
  ;[1 1 1] Press Challenges
  (CallFunction|PressChallengeButton OtherActor))

(event OnComponentBeginOverlap(Challenge1Box)
  (params (OverlappedComponent :type Primitive%20Component%20Object%20Reference) (OtherActor :type Actor%20Object%20Reference) (OtherComp :type Primitive%20Component%20Object%20Reference) (OtherBodyIndex :type Integer) (bFromSweep :type Boolean) (SweepResult :type Hit%20Result%20Structure%20%28by%20ref%29))
  ;[1 1 1] Challenge1
  (if (and (Actor|ActorHasTag OtherActor "Hand") (Variables|Challenges|GetInChallengeMenu))
    (Variables|Challenges|SetChallenge1Select true)
    (Rendering|SetVisibility (Variables|Default|GetValidChallengeButton) true false)))

(event OnComponentBeginOverlap(ValidChallengeButtonBox)
  (params (OverlappedComponent :type Primitive%20Component%20Object%20Reference) (OtherActor :type Actor%20Object%20Reference) (OtherComp :type Primitive%20Component%20Object%20Reference) (OtherBodyIndex :type Integer) (bFromSweep :type Boolean) (SweepResult :type Hit%20Result%20Structure%20%28by%20ref%29))
  ;[1 1 1] Valid Challenge
  (if (Actor|ActorHasTag OtherActor "Hand")
    (if (Variables|Challenges|GetChallenge1Select)
      (Variables|/Game/PFE/Blueprint/GameInstance/GameInstance_PFE.GameInstance_PFE_C|SetChallenge1Active (Variables|Default|GetGI) true)
      (Variables|Challenges|SetInChallengeMenu false)
      (CallFunction|Clear))))

(event OnComponentBeginOverlap(ReturnButtonBox)
  (params (OverlappedComponent :type Primitive%20Component%20Object%20Reference) (OtherActor :type Actor%20Object%20Reference) (OtherComp :type Primitive%20Component%20Object%20Reference) (OtherBodyIndex :type Integer) (bFromSweep :type Boolean) (SweepResult :type Hit%20Result%20Structure%20%28by%20ref%29))
  (if (Actor|ActorHasTag OtherActor "Hand")
    (if (or (Variables|Upgrade|GetInUpgradeP1) (Variables|Upgrade|GetInUpgradeP2))
      (Rendering|SetVisibility (Variables|Default|GetP2Button) true false)
      (Variables|Upgrade|SetInUpgradeMenu true)
      (Collision|SetCollisionEnabled (Variables|Default|GetP2ButtonBox) "QueryOnly")
      (Variables|Upgrade|SetInUpgradeP1 false)
      (Variables|Upgrade|SetInUpgradeP2 false)
      (Variables|Upgrade|SetLifeButtonP1 false)
      (Variables|Upgrade|SetLifeButtonP2 false)
      (Rendering|SetVisibility (Variables|Default|GetLifeUpgradeButton) false false)
      (Collision|SetCollisionEnabled (Variables|Default|GetLifeUpgradeButtonBox) "NoCollision")
      (else
        (Rendering|SetVisibility (Variables|Default|GetMissionMenu) true false)
        (Rendering|SetVisibility (Variables|Default|GetMission1) false false)
        (Collision|SetCollisionEnabled (Variables|Default|GetP2ButtonBox) "NoCollision")
        (Variables|Challenges|SetInChallengeMenu false)
        (Variables|Missions|SetInMissionMenu false)
        (Collision|SetCollisionEnabled (Variables|Default|GetMissionMenuBox) "QueryOnly")
        (Variables|Missions|SetMissionValid false)
        (Variables|Upgrade|SetInUpgradeMenu false)))))

(event OnComponentBeginOverlap(UpgradeMenuBox)
  (params (OverlappedComponent :type Primitive%20Component%20Object%20Reference) (OtherActor :type Actor%20Object%20Reference) (OtherComp :type Primitive%20Component%20Object%20Reference) (OtherBodyIndex :type Integer) (bFromSweep :type Boolean) (SweepResult :type Hit%20Result%20Structure%20%28by%20ref%29))
  ;[1 1 1] Press Upgrade
  (CallFunction|PressUpgradeButton OtherActor))

(event OnComponentBeginOverlap(P1ButtonBox)
  (params (OverlappedComponent :type Primitive%20Component%20Object%20Reference) (OtherActor :type Actor%20Object%20Reference) (OtherComp :type Primitive%20Component%20Object%20Reference) (OtherBodyIndex :type Integer) (bFromSweep :type Boolean) (SweepResult :type Hit%20Result%20Structure%20%28by%20ref%29))
  ;[1 1 1] Press P1Button
  (CallFunction|PressP1UpgradeButton OtherActor))

(event OnComponentBeginOverlap(LifeUpgradeButtonBox)
  (params (OverlappedComponent :type Primitive%20Component%20Object%20Reference) (OtherActor :type Actor%20Object%20Reference) (OtherComp :type Primitive%20Component%20Object%20Reference) (OtherBodyIndex :type Integer) (bFromSweep :type Boolean) (SweepResult :type Hit%20Result%20Structure%20%28by%20ref%29))
  (CallFunction|PressLifeUpgradeP1Button OtherActor))

(event Custom|Clear
  (if (Actor|ActorHasTag (stale OnComponentBeginOverlap(ReturnButtonBox) OtherActor) "Hand")
    (if (or (Variables|Upgrade|GetInUpgradeP1) (Variables|Upgrade|GetInUpgradeP2))
      (Rendering|SetVisibility (Variables|Default|GetP2Button) true false)
      (Variables|Upgrade|SetInUpgradeMenu true)
      (Collision|SetCollisionEnabled (Variables|Default|GetP2ButtonBox) "QueryOnly")
      (Variables|Upgrade|SetInUpgradeP1 false)
      (Variables|Upgrade|SetInUpgradeP2 false)
      (Variables|Upgrade|SetLifeButtonP1 false)
      (Variables|Upgrade|SetLifeButtonP2 false)
      (Rendering|SetVisibility (Variables|Default|GetLifeUpgradeButton) false false)
      (Collision|SetCollisionEnabled (Variables|Default|GetLifeUpgradeButtonBox) "NoCollision")
      (else
        (Rendering|SetVisibility (Variables|Default|GetMissionMenu) true false)
        (Rendering|SetVisibility (Variables|Default|GetMission1) false false)
        (Collision|SetCollisionEnabled (Variables|Default|GetP2ButtonBox) "NoCollision")
        (Variables|Challenges|SetInChallengeMenu false)
        (Variables|Missions|SetInMissionMenu false)
        (Collision|SetCollisionEnabled (Variables|Default|GetMissionMenuBox) "QueryOnly")
        (Variables|Missions|SetMissionValid false)
        (Variables|Upgrade|SetInUpgradeMenu false)))))

(event Custom|PressMissionButton
  (params (Target :type Actor%20Object%20Reference))
  ;[1 1 1] MissionButtonEvent
  (if (Math|Boolean|ANDBoolean (Actor|ActorHasTag Target "Hand") (not (Variables|Missions|GetInMissionMenu)) (not (Variables|Challenges|GetInChallengeMenu)))
    (Rendering|SetVisibility (Variables|Default|GetMissionMenu) false false)
    (Rendering|SetVisibility (Variables|Default|GetMission1) true false)
    (Collision|SetCollisionEnabled (Variables|Default|GetUpgradeMenuBox) "NoCollision")
    (Utilities|FlowControl|Delay 0.5)
    (Variables|Missions|SetInMissionMenu true)))

(event Custom|Loading%20Screen
  (bind _returnvalue (UserInterface|CreateWidget "/Game/PFE/Blueprint/Widget/LoadingScreen.LoadingScreen_C"))
  (UserInterface|Viewport|AddtoViewport _returnvalue 0)
  (Utilities|FlowControl|Delay 0.2))

(event Custom|PressLifeUpgradeP1Button
  (params (Target :type Actor%20Object%20Reference))
  (if (and (Actor|ActorHasTag Target "Hand") (Variables|Upgrade|GetInUpgradeP1))
    (Utilities|FlowControl|Delay 0.5)
    (Collision|SetCollisionEnabled (Variables|Default|GetLifeUpgradeButtonBox) "NoCollision")
    (Variables|Upgrade|SetLifeButtonP1 true)
    (Rendering|SetVisibility (Variables|Default|GetValidUpgradeButton) true false)
    (Collision|SetCollisionEnabled (Variables|Default|GetValidUpgradeButtonBox) "QueryOnly")))

(event Custom|CalculateLifeUpgradeP2
  (bind _gi (Variables|Default|GetGI))
  (if (and (Variables|/Game/PFE/Blueprint/GameInstance/GameInstance_PFE.GameInstance_PFE_C|GetLifeP2Level1 _gi) (>= (Variables|/Game/PFE/Blueprint/GameInstance/GameInstance_PFE.GameInstance_PFE_C|GetMoney _gi) 3))
    (Variables|/Game/PFE/Blueprint/GameInstance/GameInstance_PFE.GameInstance_PFE_C|SetLifeP2Level2 _gi true)
    (Variables|/Game/PFE/Blueprint/GameInstance/GameInstance_PFE.GameInstance_PFE_C|SetLifeP2Level1 _gi false)
    (Variables|/Game/PFE/Blueprint/J2/Player2.Player2_C|SetLife (Variables|Default|GetP2) 1.2e+02)
    (elif (and (Variables|/Game/PFE/Blueprint/GameInstance/GameInstance_PFE.GameInstance_PFE_C|GetLifeP2Level2 _gi) (>= (Variables|/Game/PFE/Blueprint/GameInstance/GameInstance_PFE.GameInstance_PFE_C|GetMoney _gi) 6))
      (Variables|/Game/PFE/Blueprint/GameInstance/GameInstance_PFE.GameInstance_PFE_C|SetLifeP2Level2 _gi false)
      (Variables|/Game/PFE/Blueprint/GameInstance/GameInstance_PFE.GameInstance_PFE_C|SetLifeP2Level3 _gi true)
      (Variables|/Game/PFE/Blueprint/J2/Player2.Player2_C|SetLife (Variables|Default|GetP2) 1.5e+02)
      (elif (and (Variables|/Game/PFE/Blueprint/GameInstance/GameInstance_PFE.GameInstance_PFE_C|GetLifeP2Level3 _gi) (>= (Variables|/Game/PFE/Blueprint/GameInstance/GameInstance_PFE.GameInstance_PFE_C|GetMoney _gi) 12))
        (Variables|/Game/PFE/Blueprint/GameInstance/GameInstance_PFE.GameInstance_PFE_C|SetLifeP2Level3 _gi false)
        (Variables|/Game/PFE/Blueprint/GameInstance/GameInstance_PFE.GameInstance_PFE_C|SetLifeP2Level4 _gi true)
        (Variables|/Game/PFE/Blueprint/J2/Player2.Player2_C|SetLife (Variables|Default|GetP2) 1.9e+02)
        (elif (and (Variables|/Game/PFE/Blueprint/GameInstance/GameInstance_PFE.GameInstance_PFE_C|GetLifeP2Level4 _gi) (>= (Variables|/Game/PFE/Blueprint/GameInstance/GameInstance_PFE.GameInstance_PFE_C|GetMoney _gi) 25))
          (Variables|/Game/PFE/Blueprint/GameInstance/GameInstance_PFE.GameInstance_PFE_C|SetLifeP2Level4 _gi false)
          (Variables|/Game/PFE/Blueprint/GameInstance/GameInstance_PFE.GameInstance_PFE_C|SetLifeP2Level5 _gi false)
          (Variables|/Game/PFE/Blueprint/J2/Player2.Player2_C|SetLife (Variables|Default|GetP2) 2.4e+02))))))

(event Custom|PressChallengeButton
  (params (Target :type Actor%20Object%20Reference))
  (bind _gi (Variables|Default|GetGI))
  ;[1 1 1] Press Challenge Button Event
  (if (Math|Boolean|ANDBoolean (Actor|ActorHasTag Target "Hand") (not (Variables|/Game/PFE/Blueprint/GameInstance/GameInstance_PFE.GameInstance_PFE_C|GetChallenge1Valid _gi)) (not (Variables|/Game/PFE/Blueprint/GameInstance/GameInstance_PFE.GameInstance_PFE_C|GetChallenge1Active _gi)))
    (Rendering|SetVisibility (Variables|Default|GetMissionMenu) false false)
    (Rendering|SetVisibility (Variables|Default|GetChallenge1Button) true false)
    (Variables|Challenges|SetInChallengeMenu true)))

(event Custom|ChangeLevel
  ;[1 1 1] Launch Mission
  (Development|ExecuteConsoleCommand (Variables|Default|GetMissionToLaunch) 0)
  (Variables|Missions|SetInMissionMenu false)
  (bind _returnvalue (Rendering|Material|CreateDynamicMaterialInstance (Variables|Default|GetStaticMesh) 0 "/Game/Test/HolographicPannelMenu.HolographicPannelMenu" "None" :!class /Script/Engine.PrimitiveComponent))
  (Rendering|Material|SetVectorParameterValue _returnvalue "Color" "(R=0.000000,G=1.000000,B=0.005394,A=1.000000)" :!class /Script/Engine.MaterialInstanceDynamic))

(event Custom|PressUpgradeButton
  (params (Target :type Actor%20Object%20Reference))
  ;[1 1 1] PressUpgradeButton
  (if (Actor|ActorHasTag Target "Hand")
    (Rendering|SetVisibility (Variables|Default|GetChallengesMenu) false false)
    (Collision|SetCollisionEnabled (Variables|Default|GetUpgradeMenuBox) "NoCollision")
    (Collision|SetCollisionEnabled (Variables|Default|GetP1ButtonBox) "QueryOnly")
    (Rendering|SetVisibility (Variables|Default|GetP2Button) true false)
    (Utilities|FlowControl|Delay 0.5)
    (Variables|Upgrade|SetInUpgradeMenu true)))

(event Custom|PressP2UpgradeButton
  (params (Target :type Actor%20Object%20Reference))
  (if (and (Actor|ActorHasTag Target "Hand") (Variables|Upgrade|GetInUpgradeMenu))
    (Rendering|SetVisibility (Variables|Default|GetLifeUpgradeP2Button) true false)
    (Collision|SetCollisionEnabled (Variables|Default|GetLiffeUpgradeP2ButtonBox) "QueryOnly")
    (Collision|SetCollisionEnabled (Variables|Default|GetP2ButtonBox) "NoCollision")
    (Rendering|SetVisibility (Variables|Default|GetP2Button) false false)
    (Variables|Upgrade|SetInUpgradeMenu false)
    (Utilities|FlowControl|Delay 0.5)
    (Variables|Upgrade|SetInUpgradeP2 true)))

(event Custom|PressLifeUpgradeP2Button
  (params (Target :type Actor%20Object%20Reference))
  (if (and (Actor|ActorHasTag Target "Hand") (Variables|Upgrade|GetInUpgradeP2))
    (Utilities|FlowControl|Delay 0.5)
    (Collision|SetCollisionEnabled (Variables|Default|GetLiffeUpgradeP2ButtonBox) "NoCollision")
    (Variables|Upgrade|SetLifeButtonP2 true)
    (Rendering|SetVisibility (Variables|Default|GetValidUpgradeButton) true false)
    (Collision|SetCollisionEnabled (Variables|Default|GetValidUpgradeButtonBox) "QueryOnly")))

(event Custom|ValidUpgradeButtonEvent
  (params (Target :type Actor%20Object%20Reference))
  (if (and (Actor|ActorHasTag Target "Hand") (or (Variables|Upgrade|GetInUpgradeP1) (Variables|Upgrade|GetInUpgradeP2)))
    (if (Variables|Upgrade|GetLifeButtonP1)
      (CallFunction|CalculateLifeUpgradeP1)
      (Variables|Upgrade|SetLifeButtonP1 false)
      (Collision|SetCollisionEnabled (Variables|Default|GetLifeUpgradeButtonBox) "QueryOnly")
      (Rendering|SetVisibility (Variables|Default|GetValidUpgradeButton) false false)
      (Collision|SetCollisionEnabled (Variables|Default|GetValidUpgradeButtonBox) "NoCollision")
      (elif (Variables|Upgrade|GetLifeButtonP2)
        (CallFunction|CalculateLifeUpgradeP2)
        (Variables|Upgrade|SetLifeButtonP2 false)
        (Collision|SetCollisionEnabled (Variables|Default|GetLiffeUpgradeP2ButtonBox) "QueryOnly")
        (Rendering|SetVisibility (Variables|Default|GetValidUpgradeButton) false false)
        (Collision|SetCollisionEnabled (Variables|Default|GetValidUpgradeButtonBox) "NoCollision")))))

(event Custom|CalculateLifeUpgradeP1
  (bind _gi (Variables|Default|GetGI))
  (if (and (Variables|/Game/PFE/Blueprint/GameInstance/GameInstance_PFE.GameInstance_PFE_C|GetLifeLevel1 _gi) (>= (Variables|/Game/PFE/Blueprint/GameInstance/GameInstance_PFE.GameInstance_PFE_C|GetMoney _gi) 3))
    (Variables|/Game/PFE/Blueprint/GameInstance/GameInstance_PFE.GameInstance_PFE_C|SetLifeLevel2 _gi true)
    (Variables|/Game/PFE/Blueprint/GameInstance/GameInstance_PFE.GameInstance_PFE_C|SetLifeLevel1 _gi false)
    (Variables|/Game/PFE/Blueprint/GameInstance/GameInstance_PFE.GameInstance_PFE_C|SetLife _gi 1.05e+03)
    (elif (and (Variables|/Game/PFE/Blueprint/GameInstance/GameInstance_PFE.GameInstance_PFE_C|GetLifeLevel2 _gi) (>= (Variables|/Game/PFE/Blueprint/GameInstance/GameInstance_PFE.GameInstance_PFE_C|GetMoney _gi) 6))
      (Variables|/Game/PFE/Blueprint/GameInstance/GameInstance_PFE.GameInstance_PFE_C|SetLifeLevel3 _gi true)
      (Variables|/Game/PFE/Blueprint/GameInstance/GameInstance_PFE.GameInstance_PFE_C|SetLifeLevel2 _gi false)
      (Variables|/Game/PFE/Blueprint/GameInstance/GameInstance_PFE.GameInstance_PFE_C|SetLife _gi 1.1e+03)
      (elif (and (Variables|/Game/PFE/Blueprint/GameInstance/GameInstance_PFE.GameInstance_PFE_C|GetLifeLevel3 _gi) (>= (Variables|/Game/PFE/Blueprint/GameInstance/GameInstance_PFE.GameInstance_PFE_C|GetMoney _gi) 12))
        (Variables|/Game/PFE/Blueprint/GameInstance/GameInstance_PFE.GameInstance_PFE_C|SetLifeLevel4 _gi true)
        (Variables|/Game/PFE/Blueprint/GameInstance/GameInstance_PFE.GameInstance_PFE_C|SetLifeLevel3 _gi false)
        (Variables|/Game/PFE/Blueprint/GameInstance/GameInstance_PFE.GameInstance_PFE_C|SetLife _gi 1.2e+03)
        (elif (and (Variables|/Game/PFE/Blueprint/GameInstance/GameInstance_PFE.GameInstance_PFE_C|GetLifeLevel4 _gi) (>= (Variables|/Game/PFE/Blueprint/GameInstance/GameInstance_PFE.GameInstance_PFE_C|GetMoney _gi) 25))
          (Variables|/Game/PFE/Blueprint/GameInstance/GameInstance_PFE.GameInstance_PFE_C|SetLifeLevel5 _gi true)
          (Variables|/Game/PFE/Blueprint/GameInstance/GameInstance_PFE.GameInstance_PFE_C|SetLifeLevel4 _gi false)
          (Variables|/Game/PFE/Blueprint/GameInstance/GameInstance_PFE.GameInstance_PFE_C|SetLife _gi 1.45e+03))))))

(event Custom|PressP1UpgradeButton
  (params (Target :type Actor%20Object%20Reference))
  ;[1 1 1] Press P1Button Event
  (if (and (Actor|ActorHasTag Target "Hand") (Variables|Upgrade|GetInUpgradeMenu))
    (Rendering|SetVisibility (Variables|Default|GetLifeUpgradeButton) true false)
    (Collision|SetCollisionEnabled (Variables|Default|GetLifeUpgradeButtonBox) "QueryOnly")
    (Collision|SetCollisionEnabled (Variables|Default|GetP2ButtonBox) "NoCollision")
    (Rendering|SetVisibility (Variables|Default|GetP2Button) false false)
    (Variables|Upgrade|SetInUpgradeMenu false)
    (Utilities|FlowControl|Delay 0.5)
    (Variables|Upgrade|SetInUpgradeP1 true)))

(event EventBeginPlay
  (bind _asgame_instance_pfe (Utilities|Casting|CastToGameInstance_PFE (Game|GetGameInstance)))
  (Variables|Default|SetGI _asgame_instance_pfe)
  (Collision|SetCollisionEnabled (Variables|Default|GetMissionMenuBox) "QueryOnly")
  (bind _asplayer_2 (Utilities|Casting|CastToPlayer2 (Game|GetPlayerCharacter 0)))
  (Variables|Default|SetP2 _asplayer_2))

(fn ConstructionScript)

(fn OnRepMission1Valid)

(fn OnRepinMissionMenu)

(fn OnRepLifeButtonP1)